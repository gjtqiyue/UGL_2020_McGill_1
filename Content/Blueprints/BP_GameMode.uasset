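; Game mode for a two-player game that spawns and possesses a Dad character for the host and a Girl character for the joining player.
; PostLogin registers controllers, and spawn points are found by PlayerStart tag.
; The host spawn waits for the game instance's finish-loading event or a client join; later loads reset both characters to the starts.
; It also relays pause toggles and cutscene continuation to both characters.
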(event `self.ReceiveBeginPlay`
  ;[1 1 1] Spawn players after level load
  (bind _asbp_game_instance (cast `/Game/Blueprints/BP_GameInstance` (`GameplayStatics.GetGameInstance`)))
  (add `/Game/Blueprints/BP_GameInstance.FinishLoading` _asbp_game_instance (delegate `FinishLoad`)))

(event `FinishLoad`
  ;[1 1 1] Spawn players after level load
  (if (`self.LevelSet`)
    (`self.Reset Player Location`)
    (else
      (set `self.LevelSet` true)
      (`self.SpawnHost`))))

(event `self.K2_PostLogin`
  (params (NewPlayer :type "PlayerController Object Reference"))
  (bind _players (`self.Players`))
  ;[1 1 1] Register player
  (`KismetArrayLibrary.Array_AddUnique` _players NewPlayer)
  (if (== (`KismetArrayLibrary.Array_Length` _players) 1)
    (set `self.HostController` NewPlayer)
    (if (`self.LevelSet`)
      (`self.SpawnHost`))
    (else
      (bind _output_get (set `self.ClientController` NewPlayer))
      (`self.SpawnClent` _output_get))))

(event `SpawnClent`
  (params (Controller :type "PlayerController Object Reference"))
  ;[1 1 1] Spawn child on new player join
  (if (`self.HostSet`)
    (`self.GetPlayerStartPoints`)
    (else
      (`self.SpawnHost`)))
  (bind _returnvalue (`|SpawnActorFromClass` "/Game/Blueprints/Characters/BP_Character_Girl.BP_Character_Girl_C" (`self.GetTransform` (`self.ChildStart`)) "AlwaysSpawn" "OverrideRootScale" null null))
  (bind _output_get (set `self.Child` _returnvalue))
  (`Controller.Possess` Controller _output_get)
  (`/Game/Blueprints/Characters/BP_CharacterBase.SetOtherPlayer` (`self.Father`) (`self.Child`))
  (`GameplayStatics.CreatePlayer` 0 false))

(event `SpawnHost`
  ;[1 1 1] Spawn parent
  (if (not (`self.HostSet`))
    (`self.GetPlayerStartPoints`)
    (bind _returnvalue (`|SpawnActorFromClass` "/Game/Blueprints/Characters/BP_Character_Dad.BP_Character_Dad_C" (`self.GetTransform` (`self.ParentStart`)) "AlwaysSpawn" "OverrideRootScale" null null))
    (set `self.Father` _returnvalue)
    (`Controller.Possess` (`self.HostController`) _returnvalue)
    (set `self.HostSet` true)
    (`GameplayStatics.CreatePlayer` 0 false)))

(event `Reset Player Location`
  (bind _child (`self.Child`))
  (bind _father (`self.Father`))
  ;[1 1 1] Reset player location
  (`self.GetPlayerStartPoints`)
  (`self.K2_SetActorLocation` _father (`self.K2_GetActorLocation` (`self.ParentStart`)) false false)
  (`/Game/Blueprints/Characters/BP_CharacterBase.Reset Player` _father)
  (`self.K2_SetActorLocation` _child (`self.K2_GetActorLocation` (`self.ChildStart`)) false false)
  (`/Game/Blueprints/Characters/BP_CharacterBase.Reset Player` _child))

(event `TogglePause`
  ;[1 1 1] Pausing Game
  (`/Game/Blueprints/Characters/BP_CharacterBase.TogglePause` (`self.Father`))
  (`/Game/Blueprints/Characters/BP_CharacterBase.TogglePause` (`self.Child`))
  (`GameplayStatics.SetGamePaused` (not (`GameplayStatics.IsGamePaused`))))

(event `ContinueCutScene`
  ;[1 1 1] Continue Cutscene
  (`/Game/Blueprints/Characters/BP_CharacterBase.ContinueCutscene` (`self.Father`))
  (`/Game/Blueprints/Characters/BP_CharacterBase.ContinueCutscene` (`self.Child`)))

(fn `GetPlayerStartPoints`
  (bind _outactors (`GameplayStatics.GetAllActorsOfClass` "/Script/Engine.PlayerStart"))
  (bind _output_get (set `self.PlayerStartArray` _outactors))
  (for _array_element _output_get
    (if (== (`PlayerStart.PlayerStartTag` _array_element) "ChildStart")
      (set `self.ChildStart` _array_element)
      (else
        (set `self.ParentStart` _array_element)))))

(fn `OnRep_PauseGame`)

(fn `UserConstructionScript`)