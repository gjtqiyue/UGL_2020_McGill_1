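; Power-up element pickup that scatters from a spawner, then homes in on a BP_Character_Dad player to be collected.
; Spread sets a random reachable direction and vertical speed, and multicasts its material.
; Tick applies hand-rolled gravity until the element nears world Z zero and activates.
; Once active, the detection sphere sets the target for interpolated homing; the inner collider adds the type to the player and HUD, then destroys the actor.
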(event `self.DetectCollider.OnComponentBeginOverlap`
  (params (OverlappedComponent :type "PrimitiveComponent Object Reference") (OtherActor :type "Actor Object Reference") (OtherComp :type "PrimitiveComponent Object Reference") (OtherBodyIndex :type Integer) (bFromSweep :type Boolean) (SweepResult :type "HitResult Structure (by ref)"))
  ;[1 1 1] Collision detection, call corresponding power up function in player
  (if (`self.Activated`)
    (bind _asbp_character_dad (cast `/Game/Blueprints/Characters/BP_Character_Dad` OtherActor))
    (set `self.Target` _asbp_character_dad)))

(event `self.Collider.OnComponentBeginOverlap`
  (params (OverlappedComponent :type "PrimitiveComponent Object Reference") (OtherActor :type "Actor Object Reference") (OtherComp :type "PrimitiveComponent Object Reference") (OtherBodyIndex :type Integer) (bFromSweep :type Boolean) (SweepResult :type "HitResult Structure (by ref)"))
  (bind _type (`self.type`))
  ;[1 1 1] Collision detection, call corresponding power up function in player
  (if (`self.Activated`)
    (bind _asbp_character_dad (cast `/Game/Blueprints/Characters/BP_Character_Dad` OtherActor))
    (`/Game/Blueprints/Widgets/BPW_PowerUp.AddElement` (`/Game/Blueprints/Characters/BP_CharacterBase.PowerUpHUD` _asbp_character_dad) _type)
    (`CharacterBase.CollectPowerUpElement` _asbp_character_dad _type)
    (`self.K2_DestroyActor`)))

(event `Activate`
  ;[1 1 1] Activation
  (set `self.Activated` true))

(event `Deactivate`
  ;[1 1 1] Activation
  (set `self.Activated` false))

(event `self.ReceiveTick`
  (params (DeltaSeconds :type "Float (single-precision)"))
  (bind (_returnvalue_x _returnvalue_y _returnvalue_z) (`KismetMathLibrary.BreakVector` (`self.K2_GetActorLocation`)))
  (bind (_returnvalue_x_2 _returnvalue_y_2 _returnvalue_z_2) (`KismetMathLibrary.BreakVector` (`self.K2_GetActorLocation`)))
  (bind (_returnvalue_x_3 _returnvalue_y_3) (`KismetMathLibrary.BreakVector` (* (`self.Direction`) (`self.SpeedXY`))))
  (if (`self.Activated`)
    (`self.AbsorbedIfPossible` DeltaSeconds)
    (else
      ;[1 1 1] If in the air
      (if (> _returnvalue_z_2 (/ (`SphereComponent.SphereRadius` (`self.Collider`)) 2.0))
        (set `self.SpeedZ` (- (`self.SpeedZ`) 10.0))
        (bind _sweephitresult (`self.K2_SetActorLocation` (+ (`SceneComponent.K2_GetComponentLocation` (`self.Collider`)) (* (`KismetMathLibrary.MakeVector` _returnvalue_x_3 _returnvalue_y_3 (`self.SpeedZ`)) DeltaSeconds)) true))
        (if (`GameplayStatics.BreakHitResult` _sweephitresult)
          (set `self.SpeedXY` 0.0))
        ;[1 1 1] Recheck if on ground
        (if (< _returnvalue_z (`SphereComponent.SphereRadius` (`self.Collider`)))
          (`self.Activate`))))))

(event `self.ReceiveBeginPlay`)

(event `self.Spread`
  (bind (_returnvalue_x _returnvalue_y) (`KismetMathLibrary.BreakVector` (- (`NavigationSystemV1.K2_GetRandomReachablePointInRadius` (`self.K2_GetActorLocation`) (`PowerUpSpawner.SpreadRange` (`self.spawner`)) null null) (`self.K2_GetActorLocation`))))
  ;[1 1 1] Spread
  (set `self.Mat` (`self.material`))
  (set `self.Direction` (`KismetMathLibrary.Normal` (`KismetMathLibrary.MakeVector` _returnvalue_x _returnvalue_y)))
  (set `self.SpeedZ` (`KismetMathLibrary.RandomFloatInRange` (`self.SpeedZMin`) (`self.SpeedZMax`)))
  (`self.MulticastSpread`))

(event `MulticastSpread`
  ;[1 1 1] Spread
  (`PrimitiveComponent.SetMaterial` (`self.Body`) 0 (`self.Mat`)))

(fn `AbsorbedIfPossible`
  (params (DeltaTime :type "Float (double-precision)"))
  (bind _target (`self.Target`))
  (`/Engine/EditorBlueprintResources/StandardMacros.IsValid` _target
    (:`Is Valid`
      (`self.K2_SetActorLocation` (`KismetMathLibrary.VInterpTo` (`self.K2_GetActorLocation`) (`self.K2_GetActorLocation` _target) DeltaTime 5.0)))))

(fn `UserConstructionScript`)