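; A power-up element pickup that spreads out, lands and is then absorbed and collected by BP_Character_Girl.
; Spread sets the material and a random direction and launch speed; Tick moves it along a hand-rolled arc, halting horizontal motion on blocking hits and activating near world Z zero.
; Once activated, DetectCollider overlap sets the character as target for an interpolated pull, and Collider overlap adds its type to her HUD and collection, then destroys it.
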(event `self.DetectCollider.OnComponentBeginOverlap`
  (params (OverlappedComponent :type "PrimitiveComponent Object Reference") (OtherActor :type "Actor Object Reference") (OtherComp :type "PrimitiveComponent Object Reference") (OtherBodyIndex :type Integer) (bFromSweep :type Boolean) (SweepResult :type "HitResult Structure (by ref)"))
  ;[1 1 1] Check target
  (if (`self.Activated`)
    (bind _asbp_character_girl (cast `/Game/Blueprints/Characters/BP_Character_Girl` OtherActor))
    (set `self.Target` _asbp_character_girl)))

(event `Activate`
  ;[1 1 1] Activation
  (set `self.Activated` true))

(event `self.Collider.OnComponentBeginOverlap`
  (params (OverlappedComponent :type "PrimitiveComponent Object Reference") (OtherActor :type "Actor Object Reference") (OtherComp :type "PrimitiveComponent Object Reference") (OtherBodyIndex :type Integer) (bFromSweep :type Boolean) (SweepResult :type "HitResult Structure (by ref)"))
  (bind _type (`self.type`))
  ;[1 1 1] Check target
  (if (`self.Activated`)
    (bind _asbp_character_girl (cast `/Game/Blueprints/Characters/BP_Character_Girl` OtherActor))
    (`/Game/Blueprints/Widgets/BPW_PowerUp.AddElement` (`/Game/Blueprints/Characters/BP_CharacterBase.PowerUpHUD` _asbp_character_girl) _type)
    (`CharacterBase.CollectPowerUpElement` _asbp_character_girl _type)
    (`self.K2_DestroyActor`)))

(event `Deactivate`
  ;[1 1 1] Activation
  (set `self.Activated` false))

(event `self.ReceiveTick`
  (params (DeltaSeconds :type "Float (single-precision)"))
  (bind (_returnvalue_x _returnvalue_y _returnvalue_z) (`KismetMathLibrary.BreakVector` (`self.K2_GetActorLocation`)))
  (bind (_returnvalue_x_2 _returnvalue_y_2 _returnvalue_z_2) (`KismetMathLibrary.BreakVector` (`self.K2_GetActorLocation`)))
  (bind (_returnvalue_x_3 _returnvalue_y_3) (`KismetMathLibrary.BreakVector` (* (`self.Direction`) (`self.SpeedXY`))))
  (if (`self.Activated`)
    ;[1 1 1] Get absorbed by player if close enough
    (`self.AbsorbedIfPossible` DeltaSeconds)
    (else
      ;[1 1 1] Function to handle spreading path
      ;;[1 1 1] If in the air
      (if (> _returnvalue_z_2 (/ (`SphereComponent.SphereRadius` (`self.Collider`)) 2.0))
        (set `self.SpeedZMax` (- (`self.SpeedZMax`) 10.0))
        (bind _sweephitresult (`self.K2_SetActorLocation` (+ (`SceneComponent.K2_GetComponentLocation` (`self.Collider`)) (* (`KismetMathLibrary.MakeVector` _returnvalue_x_3 _returnvalue_y_3 (`self.SpeedZMax`)) DeltaSeconds)) true))
        (if (`GameplayStatics.BreakHitResult` _sweephitresult)
          (set `self.SpeedXY` 0.0))
        ;;[1 1 1] Recheck if on ground
        (if (< _returnvalue_z (`SphereComponent.SphereRadius` (`self.Collider`)))
          (`self.Activate`))))))

(event `self.Spread`
  (bind (_returnvalue_x _returnvalue_y) (`KismetMathLibrary.BreakVector` (`KismetMathLibrary.RandomUnitVector`)))
  ;[1 1 1] Spread function
  (set `self.Mat` (`self.material`))
  (set `self.Direction` (`KismetMathLibrary.Normal` (`KismetMathLibrary.MakeVector` _returnvalue_x _returnvalue_y)))
  (set `self.SpeedZMax` (`KismetMathLibrary.RandomFloatInRange` (`self.SpeedZMin`) (`self.SpeedZMax`)))
  (`PrimitiveComponent.SetMaterial` (`self.Body`) 0 (`self.Mat`)))

(fn `AbsorbedIfPossible`
  (params (DeltaTime :type "Float (double-precision)"))
  (bind _target (`self.Target`))
  ;[1 1 1] Lerp to character location
  (`/Engine/EditorBlueprintResources/StandardMacros.IsValid` _target
    (:`Is Valid`
      (`self.K2_SetActorLocation` (`KismetMathLibrary.VInterpTo` (`self.K2_GetActorLocation`) (`self.K2_GetActorLocation` _target) DeltaTime 5.0)))))

(fn `UserConstructionScript`)