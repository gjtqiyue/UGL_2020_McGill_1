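; Cutscene manager that starts scenes on the Girl and Dad characters and holds the image sequences for them.
; Tick polls until both characters exist, waits briefly, triggers the first scene, then disables itself.
; The Girl's tutorial combat start event triggers the second scene; both scenes call StartCutscene on each character.
; GetNextImage steps through nested scene and image arrays, advancing to the next scene when images run out.
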(event `self.ReceiveTick`
  (params (DeltaSeconds :type "Float (single-precision)"))
  (if (`self.initPlayers`)
    (`KismetSystemLibrary.Delay` 2.0)
    (add `/Game/Blueprints/Characters/BP_CharacterBase.TutCombatStart` (`self.Girl`) (delegate `TriggerScene2`))
    (`self.TriggerScene1`)
    (`self.SetActorTickEnabled` false)
    (else
      (bind _valid (`self.Get Players`))
      (if _valid
        (set `self.initPlayers` true)))))

(event `TriggerScene2`
  (`/Game/Blueprints/Characters/BP_CharacterBase.StartCutscene` (`self.Father`))
  (`/Game/Blueprints/Characters/BP_CharacterBase.StartCutscene` (`self.Girl`)))

(event `TriggerScene1`
  (`/Game/Blueprints/Characters/BP_CharacterBase.StartCutscene` (`self.Father`))
  (`/Game/Blueprints/Characters/BP_CharacterBase.StartCutscene` (`self.Girl`)))

(fn `Get Players`
  (returns (Valid :type Boolean))
  (bind _returnvalue (`GameplayStatics.GetActorOfClass` "/Game/Blueprints/Characters/BP_Character_Girl.BP_Character_Girl_C"))
  (`/Engine/EditorBlueprintResources/StandardMacros.IsValid` _returnvalue
    (:`Is Valid`
      (set `self.Girl` _returnvalue)
      (bind _returnvalue_2 (`GameplayStatics.GetActorOfClass` "/Game/Blueprints/Characters/BP_Character_Dad.BP_Character_Dad_C"))
      (`/Engine/EditorBlueprintResources/StandardMacros.IsValid` _returnvalue_2
        (:`Is Valid`
          (set `self.Father` _returnvalue_2)
          (return true))
        (:`Is Not Valid`
          _)))
    (:`Is Not Valid`
      _))
  (return false))

(fn `GetNextImage`
  (returns (NewParam :type "Texture Object Reference"))
  (bind _scene (`self.Scene`))
  (bind _sceneindex (`self.SceneIndex`))
  (bind _textureindex (`self.TextureIndex`))
  (bind _cutscene (break `/Game/Blueprints/LevelComponent/CutScene` (`|GetArrayItem` _scene _sceneindex)))
  (if (>= (`KismetArrayLibrary.Array_Length` _scene) _sceneindex)
    (if (>= (`KismetArrayLibrary.Array_Length` _cutscene) _textureindex)
      (bind _output_get (set `self.NextImage` (`|GetArrayItem` _cutscene _textureindex)))
      (`/Engine/EditorBlueprintResources/StandardMacros.IsValid` _output_get
        (:`Is Valid`
          (set `self.TextureIndex` (+ 1 (`self.TextureIndex`)))
          (return (`self.NextImage`)))
        (:`Is Not Valid`
          _)))
    (set `self.TextureIndex` 0)
    (set `self.SceneIndex` (+ (`self.SceneIndex`) 1))
    (return null)
    (else
      (set `self.TextureIndex` 0)
      (return null))))

(fn `UserConstructionScript`)