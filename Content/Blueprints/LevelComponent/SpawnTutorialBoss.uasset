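; Level-placed spawner that creates the tutorial boss, a BP_PullToy, when the Dad character's tutorial combat starts.
; Tick looks up BP_Character_Dad until one is valid, then binds SpawnBoss to its combat-start event once, guarded by the EventBind flag.
; SpawnBoss calls SpawnServer, which always spawns the boss at this actor's transform with Dad as instigator and prints a debug message.
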(event `self.ReceiveTick`
  (params (DeltaSeconds :type "Float (single-precision)"))
  (if (not (`self.EventBind`))
    (bind _returnvalue (`GameplayStatics.GetActorOfClass` "/Game/Blueprints/Characters/BP_Character_Dad.BP_Character_Dad_C"))
    (`/Engine/EditorBlueprintResources/StandardMacros.IsValid` _returnvalue
      (:`Is Valid`
        (add `/Game/Blueprints/Characters/BP_CharacterBase.TutCombatStart` _returnvalue (delegate `SpawnBoss`))
        (set `self.EventBind` true)))))

(event `SpawnBoss`
  (`self.SpawnServer`))

(event `SpawnServer`
  (`|SpawnActorFromClass` "/Game/Blueprints/AI/BP_PullToy.BP_PullToy_C" (`self.GetTransform`) "AlwaysSpawn" "OverrideRootScale" null (stale `self.ReceiveTick` _returnvalue))
  (`KismetSystemLibrary.PrintString` "Spawned Boss"))

(fn `UserConstructionScript`)