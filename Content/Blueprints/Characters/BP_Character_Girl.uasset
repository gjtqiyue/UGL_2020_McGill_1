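; Girl-role player character Blueprint, extending a parent character with a shooting attack and two timed power-ups.
; Attack, when not down, fires the "Shoot" skill from the Sphere's transform through paired server and owning events.
; Speed and invincibility power-ups call companion events into shared logic, then reset on timers.
; The TakeDamage override skips parent damage handling while the Invincible state flag is set.
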(event `self.ReceiveBeginPlay`
  (set `self.CharacterRole` "VE_Girl")
  (`parent.ReceiveBeginPlay`))

(event `self.Attack`
  (if (not (`self.isDown`))
    (`self.Fire_server`)
    (`self.FireOwning`)))

(event `Fire_server`
  (`SkillUsage.Fire` self "Shoot" (`SceneComponent.K2_GetComponentToWorld` (`self.Sphere`))))

(event `self.ActivateSpeedPowerUp`
  ;[1 1 1] Move speed boost up
  (`self.SpeedBoost`)
  (set `CharacterMovementComponent.MaxWalkSpeed` (* (`.moveSpeed_6_4DB037464702727E9E85E59F9812D25F` (break `/Game/Blueprints/Characters/CombatStatus` (`self.Status`))) (`self.MoveSpeedBoostRatio`)) (`self.CharacterMovement`) :!label _label)
  (`KismetSystemLibrary.K2_SetTimerDelegate` (delegate `ResetSpeed`) (`self.MoveSpeedBoostDuration`)))

(event `FireOwning`
  (`SkillUsage.Fire` self "Shoot" (`SceneComponent.K2_GetComponentToWorld` (`self.Sphere`))))

(event `SpeedBoost`
  ;[1 1 1] Move speed boost up
  (goto _label))

(event `ResetSpeed`
  ;[1 1 1] Move speed boost up
  (set `CharacterMovementComponent.MaxWalkSpeed` (`.moveSpeed_6_4DB037464702727E9E85E59F9812D25F` (break `/Game/Blueprints/Characters/CombatStatus` (`self.Status`))) (`self.CharacterMovement`)))

(event `self.ActivateInvincibilityPowerUp`
  (bind _state (`self.State`))
  ;[1 1 1] Invincibility Power UP
  (`self.ActivateInvServer`)
  (if (not (`.bInvincible_28_6B1B320D42E14A30AC848ABC66F120B2` (break `/Game/Blueprints/Characters/State` _state))) :!label _label_2
    (setmembers `/Game/Blueprints/Characters/State` :`StructRef` _state :`bInvincible` true)
    (`KismetSystemLibrary.K2_SetTimerDelegate` (delegate `ResetInvincibility`) (`self.InvincibilityPowerUpDuration`))
    (`KismetSystemLibrary.PrintString` "Invincible now!!!!")))

(event `ActivateInvServer`
  ;[1 1 1] Invincibility Power UP
  (goto _label_2))

(event `ResetInvincibility`
  ;[1 1 1] Invincibility Power UP
  (setmembers `/Game/Blueprints/Characters/State` :`StructRef` (`self.State`) :`bInvincible` false))

(fn `TakeDamage`
  (params (Damage :type "Float (double-precision)") (Attacker :type "/Game/Blueprints/AI/BP_EnemyBase Object Reference") (ApplyDirection :type "Vector Structure"))
  (if (`.bInvincible_28_6B1B320D42E14A30AC848ABC66F120B2` (break `/Game/Blueprints/Characters/State` (`self.State`)))
    (`KismetSystemLibrary.PrintString` "Im invincible")
    (else
      (`parent.TakeDamage` Damage Attacker ApplyDirection))))

(fn `UserConstructionScript`
  (`parent.UserConstructionScript`))