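; Dad player character, a melee brawler that takes one third of incoming damage and flashes its material when hit.
; Attack locks movement and advances a combo, with hit and finish events toggling the LeftHit box and a timer or uppercut resetting it.
; LeftHit overlaps damage enemies and dust bunnies and trigger interactables.
; Also provides timed attack/move speed boosts and console-command slow motion; camera zoom and arm-swing logic is unconnected.
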(event `self.ReceiveBeginPlay`
  (bind _arm (`self.Arm`))
  (`parent.ReceiveBeginPlay`)
  (`PrimitiveComponent.SetCollisionEnabled` (`self.LeftHit`) "NoCollision")
  (set `self.OriginalRotation` (`SceneComponent.RelativeRotation` _arm))
  (set `self.OriginalHitBoxArmLength` (`SpringArmComponent.TargetArmLength` _arm))
  (set `self.OriginalCameraArmLength` (`SpringArmComponent.TargetArmLength` (`self.CameraBoom`))))

(event `self.ReceiveTick`
  (params (DeltaSeconds :type "Float (single-precision)"))
  (`parent.ReceiveTick` DeltaSeconds))

(event `CheckTimer`
  (bind (_state_bpanicing _state_bhealing _state_bfinishtut _state_bstartfirstcombat _state_bincombo _state_bincombatanimation) (break `/Game/Blueprints/Characters/State` (`self.State`)))
  (if _state_bincombo
    _
    (elif (not _state_bincombatanimation)
      (setmembers `/Game/Blueprints/Characters/State` :`StructRef` (`self.State`) :`bInCombatAnimation` true)
      ;[1 1 1] If timer runs out, in combo is false, reset combo hit
      (set `self.ComboHit` 0)
      (`CharacterMovementComponent.SetMovementMode` (`self.CharacterMovement`) "MOVE_Walking" 0)
      (`KismetSystemLibrary.Delay` 0.2)
      (setmembers `/Game/Blueprints/Characters/State` :`StructRef` (`self.State`) :`bInCombatAnimation` false))))

(event `FinishHookPunch`
  ;[1 1 1] Attack (temporary)
  ;;[1 1 1] Disable collision box
  (`PrimitiveComponent.SetCollisionEnabled` (`self.LeftHit`) "NoCollision")
  (setmembers `/Game/Blueprints/Characters/State` :`StructRef` (`self.State`) :`bInCombo` false)
  (setmembers `/Game/Blueprints/Characters/State` :`StructRef` (`self.State`) :`bInCombatAnimation` false)
  (`KismetSystemLibrary.K2_SetTimerDelegate` (delegate `CheckTimer`) (`self.ComboTimerLimit`)))

(event `self.Attack`
  (bind (_state_bpanicing _state_bhealing _state_bfinishtut _state_bstartfirstcombat _state_bincombo _state_bincombatanimation _state_bfirsttimehealing _state_bfirsttimepanicing _state_bstunned _state_binvincible _state_bgettinghit) (break `/Game/Blueprints/Characters/State` (`self.State`)))
  ;[1 1 1] Attack (temporary)
  (if (`self.isDown`)
    _
    (elif _state_bgettinghit
      _
      (elif _state_bstunned
        _
        (elif _state_bincombo
          _
          (elif (not _state_bincombatanimation)
            (`CharacterMovementComponent.DisableMovement` (`self.CharacterMovement`))
            (setmembers `/Game/Blueprints/Characters/State` :`StructRef` (`self.State`) :`bInCombatAnimation` true)
            ;;[1 1 1] Start combo
            (setmembers `/Game/Blueprints/Characters/State` :`StructRef` (`self.State`) :`bInCombo` true)
            ;;[1 1 1] Increment Combo
            (`/Engine/EditorBlueprintResources/StandardMacros.IncrementInt` (`self.ComboHit`))))))))

(event `FlashMaterial`
  (`PrimitiveComponent.SetMaterial` (`self.Mesh`) 1 "/Engine/MapTemplates/Materials/BasicAsset01.BasicAsset01")
  (`KismetSystemLibrary.Delay` 0.2)
  (`PrimitiveComponent.SetMaterial` (`self.Mesh`) 1 "/Engine/MapTemplates/Materials/BasicAsset02.BasicAsset02"))

(event `FinishUpperCut`
  ;[1 1 1] Attack (temporary)
  (`PrimitiveComponent.SetCollisionEnabled` (`self.LeftHit`) "NoCollision")
  (set `self.ComboHit` 0)
  (`CharacterMovementComponent.SetMovementMode` (`self.CharacterMovement`) "MOVE_Walking" 0)
  ;;[1 1 1] Time before combo set
  (`KismetSystemLibrary.Delay` (`self.ComboWaitTime`))
  (setmembers `/Game/Blueprints/Characters/State` :`StructRef` (`self.State`) :`bInCombo` false)
  (setmembers `/Game/Blueprints/Characters/State` :`StructRef` (`self.State`) :`bInCombatAnimation` false))

(event `HitEnemy`
  ;[1 1 1] Attack (temporary)
  (`PrimitiveComponent.SetCollisionEnabled` (`self.LeftHit`) "QueryOnly"))

(event `self.LeftHit.OnComponentBeginOverlap`
  (params (OverlappedComponent :type "PrimitiveComponent Object Reference") (OtherActor :type "Actor Object Reference") (OtherComp :type "PrimitiveComponent Object Reference") (OtherBodyIndex :type Integer) (bFromSweep :type Boolean) (SweepResult :type "HitResult Structure (by ref)"))
  ;[1 1 1] Attack (temporary)
  (`|ExecutionSequence`
    (:`then_0`
      (`self.DamageToEnemy` OtherActor))
    (:`then_1`
      (bind _asbp_dust_bunny (cast `/Game/Blueprints/AI/BP_DustBunny` OtherActor))
      (`/Game/Blueprints/AI/BP_DustBunny.TakeDamage` _asbp_dust_bunny self))
    (:`then_2`
      (bind _asbp_interactable (cast `/Game/Blueprints/Interactable/BP_Interactable` OtherActor))
      (`/Game/Blueprints/Interactable/BP_Interactable.GetHitByDad` _asbp_interactable))))

(event `self.LeftHit.OnComponentEndOverlap`
  (params (OverlappedComponent :type "PrimitiveComponent Object Reference") (OtherActor :type "Actor Object Reference") (OtherComp :type "PrimitiveComponent Object Reference") (OtherBodyIndex :type Integer))
  ;[1 1 1] Attack (temporary)
)

(event `ActivateSlowMotion`
  ;[1 1 1] Slow motion and zoom on camera
  (`KismetSystemLibrary.ExecuteConsoleCommand` (`KismetStringLibrary.BuildString_Double` "" "slomo " (`self.SlowMotionRate`)) null))

(event `DeactivateSlowMotion`
  ;[1 1 1] Slow motion and zoom on camera
  (`KismetSystemLibrary.ExecuteConsoleCommand` (`KismetStringLibrary.BuildString_Double` "" "slomo " 1.0) null))

(event `FinalBlowEffect`
  ;[1 1 1] Slow motion and zoom on camera
)

(event `self.ActivateAttackPowerUp`
  (bind _status (`self.Status`))
  ;[1 1 1] Attack speed boost
  (setmembers `/Game/Blueprints/Characters/CombatStatus` :`StructRef` _status :`attackSpeed` (* (`.attackSpeed_11_162EAB964095C8A8597E3FB115C9B5C8` (break `/Game/Blueprints/Characters/CombatStatus` _status)) (`self.AttackSpeedBoostRatio`)))
  (`KismetSystemLibrary.K2_SetTimerDelegate` (delegate `AttackBoost`) (`self.AttackSpeedBoostDuration`)))

(event `self.ActivateSpeedPowerUp`
  ;[1 1 1] Move speed boost up
  (set `CharacterMovementComponent.MaxWalkSpeed` (* (`.moveSpeed_6_4DB037464702727E9E85E59F9812D25F` (break `/Game/Blueprints/Characters/CombatStatus` (`self.Status`))) (`self.MoveSpeedBoostRatio`)) (`self.CharacterMovement`))
  (`KismetSystemLibrary.K2_SetTimerDelegate` (delegate `ResetSpeed`) (`self.MoveSpeedBoostDuration`)))

(event `AttackBoost`
  (bind _status (`self.Status`))
  ;[1 1 1] Attack speed boost
  (setmembers `/Game/Blueprints/Characters/CombatStatus` :`StructRef` _status :`attackSpeed` (/ (`.attackSpeed_11_162EAB964095C8A8597E3FB115C9B5C8` (break `/Game/Blueprints/Characters/CombatStatus` _status)) (`self.AttackSpeedBoostRatio`))))

(event `ResetSpeed`
  ;[1 1 1] Move speed boost up
  (set `CharacterMovementComponent.MaxWalkSpeed` (`.moveSpeed_6_4DB037464702727E9E85E59F9812D25F` (break `/Game/Blueprints/Characters/CombatStatus` (`self.Status`))) (`self.CharacterMovement`)))

(fn `CheckComboTimer`
  (params (DeltaSecond :type "Float (double-precision)")))

(fn `DamageToEnemy`
  (params (Object :type "Object Object Reference"))
  (bind _asbp_enemy_base (cast `/Game/Blueprints/AI/BP_EnemyBase` Object))
  (`self.CameraShake`)
  (`/Game/Blueprints/AI/BP_EnemyBase.TakeDamage` _asbp_enemy_base 0.0 self (`self.ComboHit`)))

(fn `ResetCombo`
  (set `self.ComboHit` 0)
  (`CharacterMovementComponent.SetMovementMode` (`self.CharacterMovement`) "MOVE_Walking" 0)
  (setmembers `/Game/Blueprints/Characters/State` :`StructRef` (`self.State`) :`bInCombo` false)
  (setmembers `/Game/Blueprints/Characters/State` :`StructRef` (`self.State`) :`bInCombatAnimation` false))

(fn `TakeDamage`
  (params (Damage :type "Float (double-precision)") (Attacker :type "/Game/Blueprints/AI/BP_EnemyBase Object Reference") (ApplyDirection :type "Vector Structure"))
  (`parent.TakeDamage` (/ Damage 3.0) Attacker ApplyDirection)
  (`self.FlashMaterial`))

(fn `UserConstructionScript`
  (`parent.UserConstructionScript`))