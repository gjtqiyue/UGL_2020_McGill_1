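; Girl player character Blueprint that manages its own health and heals while near other characters.
; BeginPlay sets the Girl role, creates the HUD showing it, then calls the parent BeginPlay.
; While not at full health, Tick scans all CharacterBase actors and adds DeltaSeconds of health for each other one within HealingDistance.
; AddHealth clamps health between zero and MaxHealth; Left Ctrl applies test damage, and debug prints remain.
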(event `self.ReceiveBeginPlay`
  (set `self.CharacterRole` "VE_Girl")
  ;[1 1 1] Adding HUD
  (bind _returnvalue (`|CreateWidget` "/Game/Blueprints/Widgets/BPW_HUD.BPW_HUD_C" (`GameplayStatics.GetPlayerController` 0)))
  (bind _output_get (set `self.HUD` _returnvalue))
  (`/Engine/EditorBlueprintResources/StandardMacros.IsValid` _output_get
    (:`Is Valid`
      (if (not (`Widget.IsInViewport` (`self.HUD`)))
        (`UserWidget.AddToViewport` _output_get 0)
        (`/Game/Blueprints/Widgets/BPW_HUD.Set RoleString` (`self.HUD`) (`|GetEnumeratorNameAsString` (`self.CharacterRole`)))
        (`parent.ReceiveBeginPlay`)))))

(event `Key|LeftControl`
  (params (Key :type "Key Structure"))
  ;[1 1 1] Test lose health
  (:`Pressed`
    (bind _newhealth (`self.AddHealth` -10.0))
    (`KismetSystemLibrary.PrintString` (`KismetStringLibrary.Conv_DoubleToString` _newhealth))))

(event `self.ReceiveTick`
  (params (DeltaSeconds :type "Float (single-precision)"))
  ;[1 1 1] Healing within distance of other player
  (if (!= (`self.Health`) (`self.MaxHealth`))
    (bind _outactors (`GameplayStatics.GetAllActorsOfClass` "/Script/McGill_1.CharacterBase"))
    (for _array_element _outactors
      (if (!= _array_element self)
        (if (< (`self.GetDistanceTo` _array_element) (`self.HealingDistance`))
          (`KismetSystemLibrary.PrintString` "In range for healing")
          (`self.AddHealth` DeltaSeconds))))))

(fn `AddHealth`
  (params (HealthChange :type "Float (double-precision)"))
  (returns (NewHealth :type "Float (double-precision)"))
  (bind _output_get (set `self.Health` (`KismetMathLibrary.FClamp` (+ HealthChange (`self.Health`)) 0.0 (`self.MaxHealth`))))
  (return _output_get))

(fn `GetHealth`
  (returns (Health :type "Float (double-precision)"))
  (return (`self.Health`)))

(fn `GetMaxHealth`
  (returns (MaxHealth :type "Float (double-precision)"))
  (return (`self.MaxHealth`)))

(fn `UserConstructionScript`)