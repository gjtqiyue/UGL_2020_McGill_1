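; Sock monkey enemy whose attack is a computed arcing leap at a target location.
; BeginPlay applies the shield material and writes safe and attack distances to the Blackboard.
; The Hit collider is enabled from launch to landing, damaging overlapped characters along the launch direction.
; Taking damage flags the AI Blackboard and plays shield-aware punch sounds for Father attackers, while death requests Father power-ups, spawned only on the server.
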(event `self.ReceiveBeginPlay`
  (bind _returnvalue (`AIBlueprintHelperLibrary.GetBlackboard` (`self.GetController`)))
  (`parent.ReceiveBeginPlay`)
  (`self.ActivateShield`)
  (`PrimitiveComponent.SetCollisionEnabled` (`self.Hit`) "NoCollision")
  (set `CharacterMovementComponent.MaxWalkSpeed` (`self.MoveSpeed`) (`self.CharacterMovement`))
  ;[1 1 1] Set up safe and attack distance
  (`/Engine/EditorBlueprintResources/StandardMacros.IsValid` _returnvalue
    (:`Is Valid`
      (`BlackboardComponent.SetValueAsFloat` _returnvalue (`self.SafeKey`) (`self.MonkeySafeDistance`))
      (`BlackboardComponent.SetValueAsFloat` (`AIBlueprintHelperLibrary.GetBlackboard` (`self.GetController`)) (`self.AttackRangeKey`) (`self.MonkeyAttackRange`)))))

(event `self.Attack`
  (set `self.OnAttack` true)
  (`self.MonkeyJump`))

(event `MonkeyJump`
  (bind (_returnvalue_x _returnvalue_y) (`KismetMathLibrary.BreakVector` (- (`self.TargetLocation`) (`self.K2_GetActorLocation`))))
  (bind _returnvalue (`KismetMathLibrary.Vector_Distance` (`self.TargetLocation`) (`self.K2_GetActorLocation`)))
  (bind _returnvalue_2 (* (/ _returnvalue (`self.JumpHeight`)) 75.0))
  (bind (_returnvalue_x_2 _returnvalue_y_2) (`KismetMathLibrary.BreakVector` (* (`KismetMathLibrary.Normal` (`KismetMathLibrary.MakeVector` _returnvalue_x _returnvalue_y)) (`self.JumpHorizontalSpeed`))))
  ;[1 1 1] Launch monkey
  (set `self.Time` (/ _returnvalue (`self.JumpHorizontalSpeed`)))
  (`KismetSystemLibrary.PrintString` (`KismetStringLibrary.Conv_DoubleToString` _returnvalue_2))
  (set `self.OnJump` true)
  (`self.LaunchCharacter` (`KismetMathLibrary.MakeVector` _returnvalue_x_2 _returnvalue_y_2 (/ (- _returnvalue_2 (* (`KismetMathLibrary.Square` (`self.Time`)) 5.0)) (`self.Time`))) true true))

(event `self.OnLaunched`
  (params (LaunchVelocity :type "Vector Structure") (bXYOverride :type Boolean) (bZOverride :type Boolean))
  (if (`self.OnJump`)
    (if (`self.OnAttack`)
      (`PrimitiveComponent.SetCollisionEnabled` (`self.Hit`) "QueryOnly")
      (set `self.LaunchVel` LaunchVelocity))))

(event `self.OnLanded`
  (params (Hit :type "HitResult Structure (by ref)"))
  (if (`self.OnJump`)
    (if (`self.OnAttack`)
      (`KismetSystemLibrary.PrintString` "Land")
      (`PrimitiveComponent.SetCollisionEnabled` (`self.Hit`) "NoCollision")
      (set `self.OnJump` false)
      (set `self.OnAttack` false))))

(event `self.Hit.OnComponentBeginOverlap`
  (params (OverlappedComponent :type "PrimitiveComponent Object Reference") (OtherActor :type "Actor Object Reference") (OtherComp :type "PrimitiveComponent Object Reference") (OtherBodyIndex :type Integer) (bFromSweep :type Boolean) (SweepResult :type "HitResult Structure (by ref)"))
  (bind _asbp_character_base (cast `/Game/Blueprints/Characters/BP_CharacterBase` OtherActor))
  (`/Engine/EditorBlueprintResources/StandardMacros.IsValid` _asbp_character_base
    (:`Is Valid`
      (`/Game/Blueprints/Characters/BP_CharacterBase.TakeDamage` _asbp_character_base (`self.AttackPower`) self (`KismetMathLibrary.Normal` (`self.LaunchVel`))))))

(event `self.Die`
  ;[1 1 1] Death
  (`self.SpawnPowerUps` "VE_Father")
  (`self.K2_DestroyActor` (`self.GetController`))
  (`self.K2_DestroyActor`))

(event `self.SpawnPowerUps`
  (params (PlayerRole :type "EPlayerRole Enum" :default "VE_Father"))
  (`parent.SpawnPowerUps` PlayerRole)
  (switch `EPlayerRole` PlayerRole
    (:`VE_Father`
      (if (`KismetSystemLibrary.IsServer`)
        (bind _returnvalue (`|SpawnActorFromClass` "/Game/Blueprints/PowerUps/BP_PowerUpSpawner_Dad.BP_PowerUpSpawner_Dad_C" (`KismetMathLibrary.MakeTransform` (0.0 0.0 0.0)) "AlwaysSpawn" "OverrideRootScale" null null))
        (`PowerUpSpawner.SpawnPowerUp` _returnvalue (`self.K2_GetActorLocation`))
        (`self.K2_DestroyActor`)))
    (:`VE_Girl`
      (if (not (`KismetSystemLibrary.IsServer`))
        (bind _returnvalue_2 (`|SpawnActorFromClass` "/Game/Blueprints/PowerUps/BP_PowerUpSpawner_Girl.BP_PowerUpSpawner_Girl_C" (`KismetMathLibrary.MakeTransform` (0.0 0.0 0.0)) "AlwaysSpawn" "OverrideRootScale" null null))
        (`PowerUpSpawner.SpawnPowerUp` _returnvalue_2 (`self.K2_GetActorLocation`))
        (`self.K2_DestroyActor`)))))

(event `PlayHitSound`
  (params (Role :type "EPlayerRole Enum" :default "VE_Father") (PunchNum :type Integer) (Attacker :type "Actor Object Reference"))
  ;[1 1 1] Play hit sound when attack
  (switch `EPlayerRole` Role
    (:`VE_Father`
      (bind _isbroken (`self.IsShieldBroken`))
      (`self.PlayHitSoundMulticast` PunchNum _isbroken))))

(event `PlayHitSoundMulticast`
  (params (HitNum :type Integer) (ShieldIsBroken :type Boolean))
  ;[1 1 1] Play hit sound when attack
  (if ShieldIsBroken
    (switch `int` HitNum
      (:`0`
        (`GameplayStatics.PlaySoundAtLocation` "/Game/Assets/Sound/SC_Punch.SC_Punch" (`self.K2_GetActorLocation`) (struct) 1.0 1.0 0.0 null null null :!label _label))
      (:`1`
        (goto _label))
      (:`2`
        (`GameplayStatics.PlaySoundAtLocation` "/Game/Assets/Sound/SC_Punch2.SC_Punch2" (`self.K2_GetActorLocation`) (struct) 1.0 1.0 0.0 null null null))
      (:`3`
        (`GameplayStatics.PlaySoundAtLocation` "/Game/Assets/Sound/SC_Punch3.SC_Punch3" (`self.K2_GetActorLocation`) (struct) 1.0 1.0 0.0 null null null)))
    (else
      (`GameplayStatics.PlaySoundAtLocation` "/Game/Assets/Sound/SC_Punch_Shield.SC_Punch_Shield" (`self.K2_GetActorLocation`) (struct) 1.0 1.0 0.0 null null null))))

(fn `ActivateShield`
  (if (`self.Shielded`)
    (`PrimitiveComponent.SetMaterial` (`self.Mesh`) 0 "/Engine/MapTemplates/Materials/BasicAsset01.BasicAsset01")))

(fn `TakeDamage`
  (params (Damage :type "Float (double-precision)") (Player :type "/Game/Blueprints/Characters/BP_CharacterBase Object Reference") (AttackCount :type Integer))
  (bind (_asbp_enemy_controller _bsuccess) (cast `/Game/Blueprints/AI/BP_Enemy_Controller` (`self.GetController`) :!pure true))
  (`parent.TakeDamage` Damage Player AttackCount)
  (`self.PlayHitSound` (`CharacterBase.CharacterRole` Player) AttackCount Player)
  ;[1 1 1] Notify being attacked
  (if _bsuccess
    (`BlackboardComponent.SetValueAsBool` (`/Game/Blueprints/AI/BP_Enemy_Controller.BB_Ref` _asbp_enemy_controller) (`self.IsAttackedKey`) true)))

(fn `UserConstructionScript`
  (`parent.UserConstructionScript`))