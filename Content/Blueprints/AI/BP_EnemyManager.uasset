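; Enemy manager that spawns dust bunny groups at players or given locations, plus optional random formations at server start.
; Player spawns branch on character role: Father groups spawn on the server, while Kid groups go through SpawnBunniesMulticast so bunnies appear only on clients.
; The server records group references per role in DustBunnyMap.
; Location spawns create a fresh server-side group without using the map.
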(event `self.ReceiveBeginPlay`
  (if (`KismetSystemLibrary.IsServer`)
    (if (`self.randomSpawn`)
      (`self.AddRandomFormations` 2))))

(event `self.SpawnBunnyGroup`
  (params (player :type "CharacterBase Object Reference") (num :type Integer))
  (bind _returnvalue (`self.GetTransform`))
  (bind _dustbunnymap (`self.DustBunnyMap`))
  (bind _characterrole (`CharacterBase.CharacterRole` player))
  (bind (_value _returnvalue_2) (`BlueprintMapLibrary.Map_Find` _dustbunnymap _characterrole))
  (if (`KismetSystemLibrary.IsServer`)
    (switch `EPlayerRole` _characterrole
      (:`VE_Father`
        ;[1 1 1] Dad server
        (bind _returnvalue_3 (`|SpawnActorFromClass` "/Game/Blueprints/AI/BP_DustBunnyGroup.BP_DustBunnyGroup_C" _returnvalue "AlwaysSpawn" "OverrideRootScale" null null))
        (if (`KismetSystemLibrary.IsServer`)
          (if _returnvalue_2
            (`/Engine/EditorBlueprintResources/StandardMacros.IsValid` _value
              (:`Is Not Valid`
                _))
            (else
              (`BlueprintMapLibrary.Map_Add` _dustbunnymap _characterrole _returnvalue_3)))
          (`/Game/Blueprints/AI/BP_DustBunnyGroup.SpawnBunnyAtPlayer` _returnvalue_3 player num self)
          (`/Game/Blueprints/AI/BP_DustBunnyGroup.SpawnBunnyAtPlayer` _value player num self)))
      (:`VE_Girl`
        (`self.SpawnBunniesMulticast` _returnvalue null _characterrole)))))

(event `SpawnBunniesMulticast`
  (params (Transform :type "Transform Structure") (Player :type "CharacterBase Object Reference") (Role :type "EPlayerRole Enum" :default "VE_Father") (Num :type Integer))
  (bind _dustbunnymap (`self.DustBunnyMap`))
  ;[1 1 1] Girl client
  ; Store group ref in enemy map on server, but spawn bunnies on client only
  (bind _returnvalue (`|SpawnActorFromClass` "/Game/Blueprints/AI/BP_DustBunnyGroup.BP_DustBunnyGroup_C" Transform "AlwaysSpawn" "OverrideRootScale" null null))
  (if (`KismetSystemLibrary.IsServer`)
    (if (`.ReturnValue` (`BlueprintMapLibrary.Map_Find` _dustbunnymap Role))
      (`/Game/Blueprints/AI/BP_DustBunnyGroup.SpawnBunnyAtPlayer` _returnvalue Player Num self :!label _label)
      (`/Game/Blueprints/AI/BP_DustBunnyGroup.SpawnBunnyAtPlayer` (`BlueprintMapLibrary.Map_Find` _dustbunnymap Role) Player Num self)
      (else
        (`BlueprintMapLibrary.Map_Add` _dustbunnymap Role _returnvalue)))
    (else
      (goto _label))))

(event `self.SpawnBunnyGroupAtLocation`
  (params (location :type "Vector Structure") (num :type Integer))
  (if (`KismetSystemLibrary.IsServer`)
    (`self.SpawnAtLocationServer` location num)))

(event `SpawnAtLocationServer`
  (params (Location :type "Vector Structure") (Num :type Integer))
  (bind _returnvalue (`|SpawnActorFromClass` "/Game/Blueprints/AI/BP_DustBunnyGroup.BP_DustBunnyGroup_C" (`KismetMathLibrary.MakeTransform` Location) "AlwaysSpawn" "OverrideRootScale" null null))
  (`/Game/Blueprints/AI/BP_DustBunnyGroup.SpawnAtLocation` _returnvalue Location Num))

(fn `UserConstructionScript`)