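; Base enemy for two-role combat: the Kid breaks its shield and the Father knocks it around with combo hits.
; TakeDamage, gated by a short cooldown, routes Father hits to hook or uppercut launches, which update the health widget only while the shield is broken.
; Shield state lives in the AI blackboard; breaking swaps material, calls power-up spawning and starts a regen timer.
; Die and SpawnPowerUps are empty here.
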(event `self.ReceiveBeginPlay`
  (bind _bb_ref (`/Game/Blueprints/AI/BP_Enemy_Controller.BB_Ref` (cast `/Game/Blueprints/AI/BP_Enemy_Controller` (`self.GetController`) :!pure true)))
  (`self.OnSpawn`)
  (bind _asbpw_enemy_health (cast `/Game/Blueprints/Widgets/BPW_EnemyHealth` (`WidgetComponent.GetUserWidgetObject` (`self.HealthWidget`))))
  (bind _output_get (set `self.HealthWidgetRef` _asbpw_enemy_health))
  (`/Game/Blueprints/Widgets/BPW_EnemyHealth.ShowShield` _output_get (`self.Shielded`))
  (set `/Game/Blueprints/Widgets/BPW_EnemyHealth.Owner_reference` self _asbpw_enemy_health)
  (set `CharacterMovementComponent.MaxWalkSpeed` (`self.MoveSpeed`) (`self.CharacterMovement`))
  ;[1 1 1] Set up controller
  (bind _asbp_enemy_controller (cast `/Game/Blueprints/AI/BP_Enemy_Controller` (`self.GetController`)))
  (`/Game/Blueprints/AI/BP_Enemy_Controller.SetupController` _asbp_enemy_controller)
  (`/Engine/EditorBlueprintResources/StandardMacros.IsValid` _bb_ref
    (:`Is Valid`
      (`BlackboardComponent.SetValueAsBool` _bb_ref (`self.ShieldKey`) (not (`self.Shielded`))))))

(event `OnSpawn`
  ;[1 1 1] onSpawn
  (bind _returnvalue (`GameplayStatics.SpawnEmitterAttached` "/Game/Assets/ParticleSystem/Spawning.Spawning" (`self.Mesh`)))
  (`KismetSystemLibrary.Delay` 2.0)
  (`ActorComponent.K2_DestroyComponent` _returnvalue))

(event `self.ReceiveTick`
  (params (DeltaSeconds :type "Float (single-precision)"))
  (if (> (`self.DamageCD`) 0.0)
    (set `self.DamageCD` (- (`self.DamageCD`) DeltaSeconds))))

(event `SetShield`
  ;[1 1 1] Reset enemy shield when time has passed
  (if (`self.Shielded`)
    (`KismetSystemLibrary.K2_SetTimerDelegate` (delegate `Reset`) (`self.ShieldRegen`))))

(event `UpdateHealth`
  (params (Hit :type Integer))
  ;[1 1 1] Update health widget
  (`/Game/Blueprints/Widgets/BPW_EnemyHealth.UpdateHealth` (`self.HealthWidgetRef`) Hit))

(event `self.Die`)

(event `Reset`
  ;[1 1 1] Reset enemy shield when time has passed
  (`BlackboardComponent.SetValueAsBool` (`AIBlueprintHelperLibrary.GetBlackboard` (`self.GetController`)) (`self.ShieldKey`) false)
  (`BlackboardComponent.SetValueAsBool` (`/Game/Blueprints/AI/BP_Enemy_Controller.BB_Ref` (cast `/Game/Blueprints/AI/BP_Enemy_Controller` (`self.GetController`) :!pure true)) (`self.ShieldKey`) false)
  (`self.ResetShieldNotify`))

(event `ResetShieldNotify`
  ;[1 1 1] Reset enemy shield when time has passed
  (`PrimitiveComponent.SetMaterial` (`self.Mesh`) 0 "/Engine/MapTemplates/Materials/BasicAsset01.BasicAsset01")
  (`/Game/Blueprints/Widgets/BPW_EnemyHealth.ShowShield` (`self.HealthWidgetRef`) true))

(event `BreakShield`
  (bind _shieldkey (`self.ShieldKey`))
  (bind _bb_ref (`/Game/Blueprints/AI/BP_Enemy_Controller.BB_Ref` (cast `/Game/Blueprints/AI/BP_Enemy_Controller` (`self.GetController`) :!pure true)))
  (bind _returnvalue (`BlackboardComponent.GetValueAsBool` _bb_ref _shieldkey))
  ;[1 1 1] Break shield
  (if (`self.Shielded`)
    (if (`KismetSystemLibrary.IsValid` (`/Game/Blueprints/AI/BP_Enemy_Controller.BB_Ref` (cast `/Game/Blueprints/AI/BP_Enemy_Controller` (`self.GetController`) :!pure true)))
      (if (not _returnvalue)
        (`BlackboardComponent.SetValueAsBool` _bb_ref _shieldkey (not _returnvalue))
        (`self.BreakShieldNotify`)
        (`self.SetShield`)))))

(event `BreakShieldNotify`
  ;[1 1 1] Break shield
  (`PrimitiveComponent.SetMaterial` (`self.Mesh`) 0 "/Engine/MapTemplates/Materials/BasicAsset03.BasicAsset03")
  ;;[1 1 1] Spawn kid power up when shield broken
  (`self.SpawnPowerUps` "VE_Girl")
  (`/Game/Blueprints/Widgets/BPW_EnemyHealth.ShowShield` (`self.HealthWidgetRef`) false))

(event `ResetHitCount`
  ;[1 1 1] Reset hit count
  (set `self.HitCount` 0)
  (`KismetSystemLibrary.PrintString` "reset count"))

(event `SpotPlayer`
  (bind _paperflipbook (`self.PaperFlipbook`))
  ;[1 1 1] Toggle visibility of exclamation mark. Missing the connecting logic to when the enemy spots the player
  (`SceneComponent.SetVisibility` _paperflipbook true false) ; When enemy can see player, make visible
  (`KismetSystemLibrary.Delay` 1.0)
  (`SceneComponent.SetVisibility` _paperflipbook false false))

(event `SpawnPowerUps`
  (params (PlayerRole :type "EPlayerRole Enum" :default "VE_Father")))

(fn `HookDamage`
  (params (Player :type "/Game/Blueprints/Characters/BP_Character_Dad Object Reference") (HitCount :type Integer))
  (bind _returnvalue (* 2 (- (`KismetMathLibrary.Conv_IntToDouble` (- HitCount 1)) 0.5)))
  (`KismetSystemLibrary.PrintString` (`KismetStringLibrary.Conv_DoubleToString` _returnvalue))
  (`self.LaunchCharacter` (+ (* (`KismetMathLibrary.Normal` (* (`self.GetActorRightVector` Player) _returnvalue)) (`self.HookForce`)) (`KismetMathLibrary.MakeVector` 0.0 0.0 (`self.HookJumpForce`))) true true)
  (bind _isbroken (`self.IsShieldBroken`))
  (if _isbroken
    (`self.UpdateHealth` HitCount)
    ;[1 1 1] Update hit count
    (`KismetSystemLibrary.K2_SetTimerDelegate` (`|CreateDelegate` :!event `ResetHitCount`) 1.0)))

(fn `IsShieldBroken`
  (returns (IsBroken :type Boolean))
  (bind _returnvalue (`self.GetController`))
  (`/Engine/EditorBlueprintResources/StandardMacros.IsValid` _returnvalue
    (:`Is Valid`
      (return (`BlackboardComponent.GetValueAsBool` (`/Game/Blueprints/AI/BP_Enemy_Controller.BB_Ref` (cast `/Game/Blueprints/AI/BP_Enemy_Controller` _returnvalue :!pure true)) (`self.ShieldKey`))))))

(fn `TakeDamage`
  (params (Damage :type "Float (double-precision)") (Player :type "/Game/Blueprints/Characters/BP_CharacterBase Object Reference") (AttackCount :type Integer))
  (returns (Success :type Boolean))
  (if (<= (`self.DamageCD`) 0.01)
    (switch `EPlayerRole` (`CharacterBase.CharacterRole` Player)
      (:`VE_Father`
        (bind _asbp_character_dad (cast `/Game/Blueprints/Characters/BP_Character_Dad` Player))
        (switch `int` AttackCount
          (:`1`
            (`self.HookDamage` _asbp_character_dad AttackCount :!label _label))
          (:`2`
            (goto _label))
          (:`3`
            (`self.UpperCutDamage` _asbp_character_dad AttackCount))))
      (:`VE_Girl`
        (cast `/Game/Blueprints/Characters/BP_Character_Girl` Player)
        (`self.BreakShield`)))
    (set `self.DamageCD` 0.1)
    (return true)
    (else
      (return false))))

(fn `UpperCutDamage`
  (params (Player :type "/Game/Blueprints/Characters/BP_Character_Dad Object Reference") (Hit :type Integer))
  ;[1 1 1] Launch player
  (`self.LaunchCharacter` (+ (* (`KismetMathLibrary.Normal` (`self.GetActorForwardVector` Player)) (`self.UpperCutForce`)) (`KismetMathLibrary.MakeVector` 0.0 0.0 (`self.UpperCutJumpForce`))) true true)
  (bind _isbroken (`self.IsShieldBroken`))
  (if _isbroken
    (`self.UpdateHealth` Hit)
    ;[1 1 1] Update hit count
    (`/Engine/EditorBlueprintResources/StandardMacros.IncrementInt` (`self.HitCount`)
      (:`  `
        ;[1 1 1] Kill enemy on third combo\
        (if (>= 0 3)
          _)))))

(fn `UserConstructionScript`)