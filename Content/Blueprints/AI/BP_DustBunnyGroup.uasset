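; Dust bunny enemy group that spawns a swarm around a location or a locally controlled player, slowing that player.
; Each hit costs shared health, sets the run-away mode, removes random bunnies and eases the slowdown in proportion to health lost, with a timed hit cooldown.
; At zero health it boosts the player's speed, clears the remaining bunnies, removes its BP_EnemyManager map entry and destroys itself.
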(event `OnGetHit`
  (params (Player :type "/Game/Blueprints/Characters/BP_CharacterBase Object Reference"))
  (bind _amount (`self.Amount`))
  (bind _slowdownbaseratio (`self.SlowDownBaseRatio`))
  ;[1 1 1] When get hit, we will set the mode to run away state (mode == 1)
  ; When normal, the mode will be wandering around the player (mode == 0)
  (if (`self.CanGetHit`)
    (set `self.CanGetHit` false)
    (bind _result (`/Engine/EditorBlueprintResources/StandardMacros.DecrementInt` (`self.Health`))
      (:`  `
        (set `self.Target` Player)
        (set `self.Mode` 1)
        (bind _returnvalue (/ (`KismetMathLibrary.Conv_IntToDouble` _result) (`KismetMathLibrary.Conv_IntToDouble` (`self.MaxHealth`))))
        (for _index (range (+ (`KismetMathLibrary.FTrunc` (* _amount _returnvalue)) 1))
          (bind _output (`|GetArrayItem` (`self.Bunnies`) (`KismetMathLibrary.RandomIntegerInRange` 0 (- _amount _index))))
          (`/Engine/EditorBlueprintResources/StandardMacros.IsValid` _output
            (:`Is Valid`
              (`/Game/Blueprints/AI/BP_DustBunny.Disappear` _output))))
        (if (== (`self.Health`) 0)
          (`/Game/Blueprints/Characters/BP_CharacterBase.BoostUpSpeed` (`self.Target`) 1.0)
          (`KismetSystemLibrary.Delay` 2.0)
          (`self.Disappear`)
          (else
            ;;[1 1 1] Calculate slow down proportional to bunny health
            (`/Game/Blueprints/Characters/BP_CharacterBase.SlowDown` Player (+ _slowdownbaseratio (* (- 1.0 _returnvalue) (- 1.0 _slowdownbaseratio))))
            (`KismetSystemLibrary.K2_SetTimerDelegate` (delegate `CanTakeHit`) 10.0)))))))

(event `self.ReceiveBeginPlay`
  (`KismetArrayLibrary.Array_Clear` (`self.Bunnies`))
  (set `self.Health` (`self.MaxHealth`))
  (bind _returnvalue (`GameplayStatics.GetActorOfClass` "/Game/Blueprints/AI/BP_EnemyManager.BP_EnemyManager_C"))
  (set `self.SlowDownBaseRatio` (`EnemyManager.dustBunniesSlowDownRatio` _returnvalue)))

(event `CanTakeHit`
  ;[1 1 1] When get hit, we will set the mode to run away state (mode == 1)
  ; When normal, the mode will be wandering around the player (mode == 0)
  (set `self.CanGetHit` true))

(event `Disappear`
  (bind _target (`self.Target`))
  (for _array_element (`self.Bunnies`)
    (`/Engine/EditorBlueprintResources/StandardMacros.IsValid` _array_element
      (:`Is Valid`
        (`/Game/Blueprints/AI/BP_DustBunny.Disappear` _array_element))))
  (`/Engine/EditorBlueprintResources/StandardMacros.IsValid` _target
    (:`Is Valid`
      (bind _returnvalue (`GameplayStatics.GetActorOfClass` "/Game/Blueprints/AI/BP_EnemyManager.BP_EnemyManager_C"))
      (`BlueprintMapLibrary.Map_Remove` (`/Game/Blueprints/AI/BP_EnemyManager.DustBunnyMap` _returnvalue) (`CharacterBase.CharacterRole` _target))
      (`KismetSystemLibrary.Delay` 3.0)
      (`self.K2_DestroyActor`))
    (:`Is Not Valid`
      (`self.K2_DestroyActor`))))

(event `SpawnAtLocation`
  (params (Location :type "Vector Structure") (Num :type Integer))
  (bind (_returnvalue_x _returnvalue_y) (`KismetMathLibrary.BreakVector` (`KismetMathLibrary.RandomUnitVector`)))
  (bind (_returnvalue_x_2 _returnvalue_y_2) (`KismetMathLibrary.BreakVector2D` (`KismetMathLibrary.Normal2D` (`KismetMathLibrary.MakeVector2D` _returnvalue_x _returnvalue_y))))
  (bind (_returnvalue_x_3 _returnvalue_y_3) (`KismetMathLibrary.BreakVector` (+ Location (* (`KismetMathLibrary.MakeVector` _returnvalue_x_2 _returnvalue_y_2) (`KismetMathLibrary.RandomFloatInRange` 50.0 (`self.FreeSpawnRadius`))))))
  ;[1 1 1] Spawn at location
  (set `self.Amount` Num)
  (for _ (range (+ Num 1))
    (bind _returnvalue (`|SpawnActorFromClass` "/Game/Blueprints/AI/BP_DustBunny.BP_DustBunny_C" (`KismetMathLibrary.MakeTransform` (`KismetMathLibrary.MakeVector` _returnvalue_x_3 _returnvalue_y_3 5.0)) "AlwaysSpawn" "OverrideRootScale" null null))
    (`/Game/Blueprints/AI/BP_DustBunny.Activate` _returnvalue self)
    (`KismetArrayLibrary.Array_Add` (`self.Bunnies`) _returnvalue)))

(event `SpawnBunnyAtPlayer`
  (params (player :type "CharacterBase Object Reference") (num :type Integer) (Manager :type "/Game/Blueprints/AI/BP_EnemyManager Object Reference"))
  (bind _returnvalue (`self.GetTransform` player))
  (bind (_returnvalue_x _returnvalue_y) (`KismetMathLibrary.BreakVector` (`KismetMathLibrary.RandomUnitVector`)))
  ;[1 1 1] Spawn at player
  (set `self.Amount` num)
  (if (== (`self.Health`) (`self.MaxHealth`))
    (set `self.Target` (cast `/Game/Blueprints/Characters/BP_CharacterBase` player :!pure true))
    ;;[1 1 1] If bunny will show on other player's screen
    (if (`Pawn.IsLocallyControlled` (`self.Target`))
      (if (not (> (`KismetArrayLibrary.Array_Length` (`self.Bunnies`)) 0))
        (for _ (range num)
          (bind _returnvalue_2 (`|SpawnActorFromClass` "/Game/Blueprints/AI/BP_DustBunny.BP_DustBunny_C" (`KismetMathLibrary.MakeTransform` (+ (* (`KismetMathLibrary.Normal` (`KismetMathLibrary.MakeVector` _returnvalue_x _returnvalue_y)) (`KismetMathLibrary.RandomFloatInRange` 50.0 (`self.PlayerBunnySpawnRange`))) (`KismetMathLibrary.MakeVector` (.x (.location _returnvalue)) (.y (.location _returnvalue)) 5.0)) (.rotation _returnvalue) (.scale _returnvalue)) "AlwaysSpawn" "OverrideRootScale" null null))
          (`/Game/Blueprints/AI/BP_DustBunny.Activate` _returnvalue_2 self)
          (`KismetArrayLibrary.Array_Add` (`self.Bunnies`) _returnvalue_2))
        (`/Game/Blueprints/Characters/BP_CharacterBase.SlowDown` (`self.Target`) (`EnemyManager.dustBunniesSlowDownRatio` Manager))))))

(fn `UserConstructionScript`)