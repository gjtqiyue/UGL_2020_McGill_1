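; BP_PullToy is a shieldable enemy that deals damage through a Hit collider toggled by charge events.
; Attack calls an empty PreCharge; the charge movement timelines are unconnected.
; Damage writes the attacker to the AI blackboard and, for Father attackers, multicasts shield-dependent punch sounds.
; Death spawns the Dad power-up and destroys pawn and controller on the server; SpawnPowerUps also has a client-side Girl branch.
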(event `self.SpawnPowerUps`
  (params (PlayerRole :type "EPlayerRole Enum" :default "VE_Father"))
  ;[1 1 1] Spawn Power Up element
  (`parent.SpawnPowerUps` PlayerRole)
  (switch `EPlayerRole` PlayerRole
    (:`VE_Father`
      (if (`KismetSystemLibrary.IsServer`)
        (bind _returnvalue (`|SpawnActorFromClass` "/Game/Blueprints/PowerUps/BP_PowerUpSpawner_Dad.BP_PowerUpSpawner_Dad_C" (`KismetMathLibrary.MakeTransform` (0.0 0.0 0.0)) "AlwaysSpawn" "OverrideRootScale" null null))
        (`PowerUpSpawner.SpawnPowerUp` _returnvalue (`self.K2_GetActorLocation`))
        (`self.K2_DestroyActor`)))
    (:`VE_Girl`
      (if (not (`KismetSystemLibrary.IsServer`))
        (bind _returnvalue_2 (`|SpawnActorFromClass` "/Game/Blueprints/PowerUps/BP_PowerUpSpawner_Girl.BP_PowerUpSpawner_Girl_C" (`KismetMathLibrary.MakeTransform` (0.0 0.0 0.0)) "AlwaysSpawn" "OverrideRootScale" null null))
        (`PowerUpSpawner.SpawnPowerUp` _returnvalue_2 (`self.K2_GetActorLocation`))
        (`self.K2_DestroyActor`)))))

(event `self.ReceiveBeginPlay`
  (`parent.ReceiveBeginPlay`)
  (`PrimitiveComponent.SetCollisionEnabled` (`self.Hit`) "NoCollision")
  (`self.ActivateShield`))

(event `self.Attack`
  ;[1 1 1] Pulltoy attck
  (set `self.IsAttacking` true)
  (set `self.AttackLocation` (`self.K2_GetActorLocation`))
  (`self.PreCharge`))

(event `PlayHitSound`
  (params (Role :type "EPlayerRole Enum" :default "VE_Father") (PunchNum :type Integer) (Attacker :type "Actor Object Reference"))
  ;[1 1 1] Play hit sound when attack
  (switch `EPlayerRole` Role
    (:`VE_Father`
      (bind _isbroken (`self.IsShieldBroken`))
      (`self.PlayHitSoundMulticast` PunchNum _isbroken))))

(event `self.Hit.OnComponentBeginOverlap`
  (params (OverlappedComponent :type "PrimitiveComponent Object Reference") (OtherActor :type "Actor Object Reference") (OtherComp :type "PrimitiveComponent Object Reference") (OtherBodyIndex :type Integer) (bFromSweep :type Boolean) (SweepResult :type "HitResult Structure (by ref)"))
  ;[1 1 1] Pulltoy attck
  (bind _asbp_character_base (cast `/Game/Blueprints/Characters/BP_CharacterBase` OtherActor))
  (`PrimitiveComponent.SetCollisionEnabled` (`self.Hit`) "NoCollision")
  (`/Game/Blueprints/Characters/BP_CharacterBase.TakeDamage` _asbp_character_base (* (`self.AttackPower`) -1.0) self (0.0 0.0 0.0)))

(event `PlayHitSoundMulticast`
  (params (HitNum :type Integer) (ShieldIsBroken :type Boolean))
  ;[1 1 1] Play hit sound when attack
  (if ShieldIsBroken
    (switch `int` HitNum
      (:`0`
        (`GameplayStatics.PlaySoundAtLocation` "/Game/Assets/Sound/SC_Punch.SC_Punch" (`self.K2_GetActorLocation`) (struct) 1.0 1.0 0.0 null null null))
      (:`1`
        (`GameplayStatics.PlaySoundAtLocation` "/Game/Assets/Sound/SC_Punch2.SC_Punch2" (`self.K2_GetActorLocation`) (struct) 1.0 1.0 0.0 null null null))
      (:`2`
        (`GameplayStatics.PlaySoundAtLocation` "/Game/Assets/Sound/SC_Punch3.SC_Punch3" (`self.K2_GetActorLocation`) (struct) 1.0 1.0 0.0 null null null)))
    (else
      (`GameplayStatics.PlaySoundAtLocation` "/Game/Assets/Sound/SC_Punch_Shield.SC_Punch_Shield" (`self.K2_GetActorLocation`) (struct) 1.0 1.0 0.0 null null null))))

(event `PreCharge`
  ;[1 1 1] Pulltoy attck
)

(event `ChargeToPlayer`
  ;[1 1 1] Pulltoy attck
  (`KismetSystemLibrary.PrintString` "Enemy attack")
  (`PrimitiveComponent.SetCollisionEnabled` (`self.Hit`) "QueryOnly"))

(event `AfterCharge`
  ;[1 1 1] Pulltoy attck
  (`PrimitiveComponent.SetCollisionEnabled` (`self.Hit`) "NoCollision"))

(fn `ActivateShield`
  (if (`self.Shielded`)
    (`PrimitiveComponent.SetMaterial` (`self.Mesh`) 0 "/Engine/MapTemplates/Materials/BasicAsset01.BasicAsset01")))

(fn `Die`
  (`self.SpawnPowerUps` "VE_Father")
  (if (`KismetSystemLibrary.IsServer`)
    (`self.K2_DestroyActor` (`self.GetController`))
    (`self.K2_DestroyActor`)))

(fn `TakeDamage`
  (params (Damage :type "Float (double-precision)") (Player :type "/Game/Blueprints/Characters/BP_CharacterBase Object Reference") (AttackCount :type Integer))
  (bind (_asbp_enemy_controller _bsuccess) (cast `/Game/Blueprints/AI/BP_Enemy_Controller` (`self.GetController`) :!pure true))
  (bind (_asbp_enemy_controller_2 _bsuccess_2) (cast `/Game/Blueprints/AI/BP_Enemy_Controller` (`self.GetController`) :!pure true))
  (bind _success (`parent.TakeDamage` Damage Player AttackCount))
  (if _success
    (`self.PlayHitSound` (`CharacterBase.CharacterRole` Player) AttackCount)
    ;[1 1 1] Set attacker
    (if _bsuccess
      (`BlackboardComponent.SetValueAsObject` (`/Game/Blueprints/AI/BP_Enemy_Controller.BB_Ref` _asbp_enemy_controller) (`self.AttackerKey`) Player)
      ;[1 1 1] Notify being attacked
      (if _bsuccess_2
        (`BlackboardComponent.SetValueAsBool` (`/Game/Blueprints/AI/BP_Enemy_Controller.BB_Ref` _asbp_enemy_controller_2) (`self.IsAttackedKey`) true)))))

(fn `UserConstructionScript`
  (`parent.UserConstructionScript`))