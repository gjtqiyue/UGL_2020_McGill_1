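; Test variant of a pull toy AI character that overrides ActivateShield with an empty body, so that function does nothing.
; TakeDamage runs the parent logic, then writes the attacking player and an is-attacked flag to the BP_Enemy_Controller blackboard.
; BeginPlay and construction only call the parent, and a leftover material swap in ActivateShield is disconnected.
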(event `self.ReceiveBeginPlay`
  (`parent.ReceiveBeginPlay`))

(fn `ActivateShield`)

(fn `TakeDamage`
  (params (Damage :type "Float (double-precision)") (Player :type "/Game/Blueprints/Characters/BP_CharacterBase Object Reference") (AttackCount :type Integer))
  (bind (_asbp_enemy_controller _bsuccess) (cast `/Game/Blueprints/AI/BP_Enemy_Controller` (`self.GetController`) :!pure true))
  (bind (_asbp_enemy_controller_2 _bsuccess_2) (cast `/Game/Blueprints/AI/BP_Enemy_Controller` (`self.GetController`) :!pure true))
  (`parent.TakeDamage` Damage Player AttackCount)
  ;[1 1 1] Set attacker
  (if _bsuccess
    (`BlackboardComponent.SetValueAsObject` (`/Game/Blueprints/AI/BP_Enemy_Controller.BB_Ref` _asbp_enemy_controller) (`self.AttackerKey`) Player)
    ;[1 1 1] Notify being attacked
    (if _bsuccess_2
      (`BlackboardComponent.SetValueAsBool` (`/Game/Blueprints/AI/BP_Enemy_Controller.BB_Ref` _asbp_enemy_controller_2) (`self.IsAttackedKey`) true))))

(fn `UserConstructionScript`
  (`parent.UserConstructionScript`))