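; Test AI controller for enemy pawns that configures its behavior according to the controlled BP_EnemyBase's combat type: Pull Toy, Sock Monkey or Giant Bear.
; A SetupController event sets the priority target (Girl or Father), loads that type's blackboard and stores the pawn's current location as its original location.
; It then runs the matching behavior tree and signals that setup has finished.
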(event `self.SetupController`
  (bind _combattype (`/Game/Blueprints/AI/BP_EnemyBase.CombatType` (cast `/Game/Blueprints/AI/BP_EnemyBase` (`self.K2_GetPawn`) :!pure true)))
  (set `self.Mode` _combattype)
  (switch `/Game/Blueprints/AI/EM_EnemyT` _combattype
    (:`NewEnumerator1`
      ;[1 1 1] PullToy
      (set `self.PriorityTarget` "VE_Girl")
      (bind _blackboardcomponent (`self.UseBlackboard` "/Game/Blueprints/AI/PullToyBehaviour/BB_Enemy.BB_Enemy"))
      (bind _output_get (set `self.BB_Ref` _blackboardcomponent))
      (`BlackboardComponent.SetValueAsVector` _output_get (`self.OriginalLocationKey`) (`self.K2_GetActorLocation` (`self.K2_GetPawn`)))
      (`self.RunBehaviorTree` "/Game/Blueprints/AI/PullToyBehaviour/BT_EnemyTest.BT_EnemyTest")
      (`self.OnFinishSetUp`))
    (:`NewEnumerator2`
      ;[1 1 1] SockMonkey
      (set `self.PriorityTarget` "VE_Father")
      (bind _blackboardcomponent_2 (`self.UseBlackboard` "/Game/Blueprints/AI/SockMonkeyBehaviour/BB_SockMonkey.BB_SockMonkey"))
      (bind _output_get_2 (set `self.BB_Ref` _blackboardcomponent_2))
      (`BlackboardComponent.SetValueAsVector` _output_get_2 (`self.OriginalLocationKey`) (`self.K2_GetActorLocation` (`self.K2_GetPawn`)))
      (`self.RunBehaviorTree` "/Game/Blueprints/AI/SockMonkeyBehaviour/BT_SockMonkey.BT_SockMonkey")
      (`self.OnFinishSetUp`))
    (:`NewEnumerator4`
      ;[1 1 1] GiantBear
      (set `self.PriorityTarget` "VE_Girl")
      (bind _blackboardcomponent_3 (`self.UseBlackboard` "/Game/Blueprints/AI/GiantBearBehaviour/BB_GiantBear.BB_GiantBear"))
      (bind _output_get_3 (set `self.BB_Ref` _blackboardcomponent_3))
      (`BlackboardComponent.SetValueAsVector` _output_get_3 (`self.OriginalLocationKey`) (`self.K2_GetActorLocation` (`self.K2_GetPawn`)))
      (`self.RunBehaviorTree` "/Game/Blueprints/AI/GiantBearBehaviour/BT_GiantBear.BT_GiantBear")
      (`self.OnFinishSetUp`))))

(fn `UserConstructionScript`
  (`parent.UserConstructionScript`))