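; Dust bunny AI agent, a physics-simulated cube steered by forces and governed by a Parent actor's Mode and Target.
; It seeks a randomly jittered point near the target with distance-scaled force, or wanders clockwise or counterclockwise without one.
; Steer-away mode applies boosted, jittered wander until a delay resets the Parent's mode.
; Damage is forwarded to Parent, Disappear destroys it after a delay, and neighbor-avoidance logic is unwired.
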(event `self.ReceiveBeginPlay`
  (bind _returnvalue (`GameplayStatics.GetActorOfClass` "/Game/Blueprints/AI/BP_EnemyManager.BP_EnemyManager_C"))
  (set `self.Manager` _returnvalue)
  (`KismetSystemLibrary.Delay` 0.2)
  (`PrimitiveComponent.SetSimulatePhysics` (`self.Cube`) true))

(event `Activate`
  (params (Parent :type "/Game/Blueprints/AI/BP_DustBunnyGroup Object Reference"))
  (bind _output_get (set `self.Parent` Parent))
  (`/Engine/EditorBlueprintResources/StandardMacros.IsValid` _output_get
    (:`Is Valid`
      (`/Engine/EditorBlueprintResources/StandardMacros.IsValid` (`/Game/Blueprints/AI/BP_DustBunnyGroup.Target` _output_get)
        (:`Is Not Valid`
          (set `self.IsSteeringCCW` (`KismetMathLibrary.Conv_IntToBool` (`KismetMathLibrary.RandomInteger` 2))))))))

(event `self.ReceiveTick`
  (params (DeltaSeconds :type "Float (single-precision)"))
  (bind _parent (`self.Parent`))
  (switch `int` (`/Game/Blueprints/AI/BP_DustBunnyGroup.Mode` _parent)
    (:`0`
      (`/Engine/EditorBlueprintResources/StandardMacros.IsValid` (`/Game/Blueprints/AI/BP_DustBunnyGroup.Target` (`self.Parent`))
        (:`Is Valid`
          ;[1 1 1] Steering to the target
          (`self.Apply Force`))
        (:`Is Not Valid`
          ;[1 1 1] No target specified
          (if (`self.IsSteeringCCW`)
            (`self.SteerCCW`)
            (else
              (`self.SteerCW`))))))
    (:`1`
      (set `self.Speed` (* 3 (`self.MaxSpeed`)))
      (`self.SteerAway`)
      ;[1 1 1] Steering away timer
      (`KismetSystemLibrary.Delay` (`self.SteerAwayTimer`))
      (set `self.Speed` (`self.MaxSpeed`))
      (set `/Game/Blueprints/AI/BP_DustBunnyGroup.Mode` 0 _parent))))

(event `Disappear`
  (`KismetSystemLibrary.Delay` 2.0)
  (`self.K2_DestroyActor`))

(fn `Apply Force`
  (bind _maxspeed (`self.MaxSpeed`))
  (bind _returnvalue (`SceneComponent.K2_GetComponentLocation` (`self.Cube`)))
  (bind (_returnvalue_x _returnvalue_y) (`KismetMathLibrary.BreakVector` (`SceneComponent.K2_GetComponentLocation` (`self.Cube`))))
  (bind _returnvalue_2 (`SceneComponent.GetComponentVelocity` (`self.Cube`)))
  (bind _returnvalue_3 (`KismetMathLibrary.VSize` _returnvalue_2))
  (bind (_returnvalue_x_2 _returnvalue_y_2) (`KismetMathLibrary.BreakVector` (- (+ (`self.K2_GetActorLocation` (`/Game/Blueprints/AI/BP_DustBunnyGroup.Target` (`self.Parent`))) (* (`KismetMathLibrary.RandomUnitVector`) (`KismetMathLibrary.RandomFloatInRange` 0.0 (`self.SmallRadius`)))) (`KismetMathLibrary.MakeVector` _returnvalue_x _returnvalue_y))))
  (bind _returnvalue_4 (`KismetMathLibrary.MakeVector` _returnvalue_x_2 _returnvalue_y_2))
  (`PrimitiveComponent.AddForce` (`self.Cube`) (* (* (`KismetMathLibrary.Normal` _returnvalue_4) (`self.Speed`)) (`KismetMathLibrary.FClamp` (* 2 (- (/ (- (`KismetMathLibrary.VSize` _returnvalue_4) 10.0) (`self.LargeRadius`)) 0.5)) -1.0 10.0)) "None" true)
  ;[1 1 1] Clamp to max speed
  (if (> _returnvalue_3 _maxspeed)
    (`PrimitiveComponent.AddForce` (`self.Cube`) (* (`KismetMathLibrary.NegateVector` _returnvalue_2) (* 2 (- _returnvalue_3 _maxspeed))) "None" false)
    ;[1 1 1] Update rotation
    (`SceneComponent.K2_SetWorldRotation` (`self.Cube`) (`KismetMathLibrary.ComposeRotators` (`KismetMathLibrary.FindLookAtRotation` _returnvalue (+ _returnvalue (`SceneComponent.GetComponentVelocity` (`self.Cube`)))) (struct :`Yaw` -90.0)) false false)))

(fn `SteerAway`
  (bind _wanderjitter (`self.WanderJitter`))
  (bind _maxspeed (`self.MaxSpeed`))
  (bind _returnvalue (`SceneComponent.GetComponentVelocity` (`self.Cube`)))
  (bind _returnvalue_2 (`SceneComponent.GetComponentVelocity` (`self.Cube`)))
  (bind _returnvalue_3 (`KismetMathLibrary.VSize` _returnvalue))
  (`PrimitiveComponent.AddForce` (`self.Cube`) (- (* (`KismetMathLibrary.Normal` (+ _returnvalue_2 (* (`KismetMathLibrary.Normal` (`KismetMathLibrary.RotateAngleAxis` (`KismetMathLibrary.GreaterGreater_VectorRotator` (`SceneComponent.GetForwardVector` (`self.Cube`)) (struct :`Yaw` 90.0)) (`KismetMathLibrary.RandomFloatInRange` (* _wanderjitter -1.0) _wanderjitter) (0.0 0.0 1.0))) (`KismetMathLibrary.RandomFloatInRange` 0.0 (`self.WanderRadius`))))) (`self.Speed`)) _returnvalue_2) "None" false)
  ;[1 1 1] Clamp to max speed
  (if (> _returnvalue_3 _maxspeed)
    (`PrimitiveComponent.AddForce` (`self.Cube`) (* (`KismetMathLibrary.NegateVector` _returnvalue) (* 2 (- _returnvalue_3 _maxspeed))) "None" false)))

(fn `SteerCCW`
  (bind _returnvalue (`SceneComponent.K2_GetComponentLocation` (`self.Cube`)))
  (bind _returnvalue_2 (`SceneComponent.GetComponentVelocity` (`self.Cube`)))
  (`PrimitiveComponent.AddForce` (`self.Cube`) (- (* (`KismetMathLibrary.Normal` (+ _returnvalue_2 (* (`KismetMathLibrary.Normal` (`KismetMathLibrary.RotateAngleAxis` (`KismetMathLibrary.GreaterGreater_VectorRotator` (`SceneComponent.GetForwardVector` (`self.Cube`)) (struct :`Yaw` 90.0)) (`KismetMathLibrary.RandomFloatInRange` (* -1 (`self.WanderJitter`))) (0.0 0.0 1.0))) (`KismetMathLibrary.RandomFloatInRange` 0.0 (`self.WanderRadius`))))) (`self.MaxSpeed`)) _returnvalue_2) "None" false)
  (`SceneComponent.K2_SetWorldRotation` (`self.Cube`) (`KismetMathLibrary.ComposeRotators` (`KismetMathLibrary.FindLookAtRotation` _returnvalue (+ _returnvalue (`SceneComponent.GetComponentVelocity` (`self.Cube`)))) (struct :`Yaw` -90.0)) false false))

(fn `SteerCW`
  (bind _returnvalue (`SceneComponent.K2_GetComponentLocation` (`self.Cube`)))
  (bind _returnvalue_2 (`SceneComponent.GetComponentVelocity` (`self.Cube`)))
  (`PrimitiveComponent.AddForce` (`self.Cube`) (- (* (`KismetMathLibrary.Normal` (+ _returnvalue_2 (* (`KismetMathLibrary.Normal` (`KismetMathLibrary.RotateAngleAxis` (`KismetMathLibrary.GreaterGreater_VectorRotator` (`SceneComponent.GetForwardVector` (`self.Cube`)) (struct :`Yaw` 90.0)) (`KismetMathLibrary.RandomFloatInRange` 0.0 (`self.WanderJitter`)) (0.0 0.0 1.0))) (`KismetMathLibrary.RandomFloatInRange` 0.0 (`self.WanderRadius`))))) (`self.MaxSpeed`)) _returnvalue_2) "None" false)
  (`SceneComponent.K2_SetWorldRotation` (`self.Cube`) (`KismetMathLibrary.ComposeRotators` (`KismetMathLibrary.FindLookAtRotation` _returnvalue (+ _returnvalue (`SceneComponent.GetComponentVelocity` (`self.Cube`)))) (struct :`Yaw` -90.0)) false false))

(fn `TakeDamage`
  (params (Player :type "/Game/Blueprints/Characters/BP_CharacterBase Object Reference"))
  (`/Game/Blueprints/AI/BP_DustBunnyGroup.OnGetHit` (`self.Parent`) Player))

(fn `UserConstructionScript`)