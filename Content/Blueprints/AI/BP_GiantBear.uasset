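; Giant bear enemy that shows an attack-range emitter and damages every character tracked inside its Hit overlap volume.
; Taking damage sets an IsAttacked blackboard flag on its AI controller and, for Father hits, plays punch sounds varying by combo count and shield state.
; Death requests Father power-ups, spawned on the server; the spawn event also has a non-server Kid branch.
; Shielded bears get a material swap on BeginPlay.
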(event `self.ReceiveBeginPlay`
  (`parent.ReceiveBeginPlay`)
  (`self.ActivateShield`)
  (set `CharacterMovementComponent.MaxWalkSpeed` (`self.MoveSpeed`) (`self.CharacterMovement`))
  (bind _returnvalue (`GameplayStatics.SpawnEmitterAttached` "/Game/Assets/ParticleSystem/BearAttackRange.BearAttackRange" (`self.Mesh`)))
  (bind _output_get (set `self.AttackAreaEmitter` _returnvalue))
  (`KismetSystemLibrary.Delay` 0.2 :!label _label)
  (`SceneComponent.K2_SetRelativeLocation` _output_get (0.0 0.0 0.0) false false)
  (goto _label))

(event `self.Attack`
  ;[1 1 1] Attack
  (for _array_element (`self.PlayerList`)
    (`/Game/Blueprints/Characters/BP_CharacterBase.TakeDamage` _array_element (`self.AttackPower`) self (0.0 0.0 0.0))))

(event `self.SpawnPowerUps`
  (params (PlayerRole :type "EPlayerRole Enum" :default "VE_Father"))
  (`parent.SpawnPowerUps` PlayerRole)
  (switch `EPlayerRole` PlayerRole
    (:`VE_Father`
      (if (`KismetSystemLibrary.IsServer`)
        (bind _returnvalue (`|SpawnActorFromClass` "/Game/Blueprints/PowerUps/BP_PowerUpSpawner_Dad.BP_PowerUpSpawner_Dad_C" (`KismetMathLibrary.MakeTransform` (0.0 0.0 0.0)) "AlwaysSpawn" "OverrideRootScale" null null))
        (`PowerUpSpawner.SpawnPowerUp` _returnvalue (`self.K2_GetActorLocation`))
        (`self.K2_DestroyActor`)))
    (:`VE_Girl`
      (if (not (`KismetSystemLibrary.IsServer`))
        (bind _returnvalue_2 (`|SpawnActorFromClass` "/Game/Blueprints/PowerUps/BP_PowerUpSpawner_Girl.BP_PowerUpSpawner_Girl_C" (`KismetMathLibrary.MakeTransform` (0.0 0.0 0.0)) "AlwaysSpawn" "OverrideRootScale" null null))
        (`PowerUpSpawner.SpawnPowerUp` _returnvalue_2 (`self.K2_GetActorLocation`))
        (`self.K2_DestroyActor`)))))

(event `self.Hit.OnComponentBeginOverlap`
  (params (OverlappedComponent :type "PrimitiveComponent Object Reference") (OtherActor :type "Actor Object Reference") (OtherComp :type "PrimitiveComponent Object Reference") (OtherBodyIndex :type Integer) (bFromSweep :type Boolean) (SweepResult :type "HitResult Structure (by ref)"))
  ;[1 1 1] Attack
  (bind _asbp_character_base (cast `/Game/Blueprints/Characters/BP_CharacterBase` OtherActor))
  (`/Engine/EditorBlueprintResources/StandardMacros.IsValid` _asbp_character_base
    (:`Is Valid`
      (if (not (`KismetArrayLibrary.Array_Contains` (`self.PlayerList`) _asbp_character_base))
        (`KismetArrayLibrary.Array_AddUnique` (`self.PlayerList`) _asbp_character_base)))))

(event `self.Hit.OnComponentEndOverlap`
  (params (OverlappedComponent :type "PrimitiveComponent Object Reference") (OtherActor :type "Actor Object Reference") (OtherComp :type "PrimitiveComponent Object Reference") (OtherBodyIndex :type Integer))
  (bind _playerlist (`self.PlayerList`))
  ;[1 1 1] Attack
  (bind _asbp_character_base (cast `/Game/Blueprints/Characters/BP_CharacterBase` OtherActor))
  (`/Engine/EditorBlueprintResources/StandardMacros.IsValid` _asbp_character_base
    (:`Is Valid`
      (if (`KismetArrayLibrary.Array_Contains` _playerlist _asbp_character_base)
        (`KismetArrayLibrary.Array_RemoveItem` _playerlist _asbp_character_base)))))

(event `self.Die`
  ;[1 1 1] Die
  (`self.SpawnPowerUps` "VE_Father")
  (`self.K2_DestroyActor` (`self.GetController`))
  (`self.K2_DestroyActor`))

(event `PlayHitSound`
  (params (Role :type "EPlayerRole Enum" :default "VE_Father") (PunchNum :type Integer) (Attacker :type "Actor Object Reference"))
  ;[1 1 1] Play hit sound when attack
  (switch `EPlayerRole` Role
    (:`VE_Father`
      (bind _isbroken (`self.IsShieldBroken`))
      (`self.PlayHitSoundMulticast` PunchNum _isbroken))))

(event `PlayHitSoundMulticast`
  (params (HitNum :type Integer) (ShieldIsBroken :type Boolean))
  ;[1 1 1] Play hit sound when attack
  (if ShieldIsBroken
    (switch `int` HitNum
      (:`0`
        (`GameplayStatics.PlaySoundAtLocation` "/Game/Assets/Sound/SC_Punch.SC_Punch" (`self.K2_GetActorLocation`) (struct) 1.0 1.0 0.0 null null null :!label _label_2))
      (:`1`
        (goto _label_2))
      (:`2`
        (`GameplayStatics.PlaySoundAtLocation` "/Game/Assets/Sound/SC_Punch2.SC_Punch2" (`self.K2_GetActorLocation`) (struct) 1.0 1.0 0.0 null null null))
      (:`3`
        (`GameplayStatics.PlaySoundAtLocation` "/Game/Assets/Sound/SC_Punch3.SC_Punch3" (`self.K2_GetActorLocation`) (struct) 1.0 1.0 0.0 null null null)))
    (else
      (`GameplayStatics.PlaySoundAtLocation` "/Game/Assets/Sound/SC_Punch_Shield.SC_Punch_Shield" (`self.K2_GetActorLocation`) (struct) 1.0 1.0 0.0 null null null))))

(fn `ActivateShield`
  (if (`self.Shielded`)
    (`PrimitiveComponent.SetMaterial` (`self.Mesh`) 0 "/Engine/MapTemplates/Materials/BasicAsset01.BasicAsset01")))

(fn `TakeDamage`
  (params (Damage :type "Float (double-precision)") (Player :type "/Game/Blueprints/Characters/BP_CharacterBase Object Reference") (AttackCount :type Integer))
  (bind (_asbp_enemy_controller _bsuccess) (cast `/Game/Blueprints/AI/BP_Enemy_Controller` (`self.GetController`) :!pure true))
  (`parent.TakeDamage` Damage Player AttackCount)
  (`self.PlayHitSound` (`CharacterBase.CharacterRole` Player) AttackCount Player)
  ;[1 1 1] Notify being attacked
  (if _bsuccess
    (`BlackboardComponent.SetValueAsBool` (`/Game/Blueprints/AI/BP_Enemy_Controller.BB_Ref` _asbp_enemy_controller) (`self.IsAttackedKey`) true)))

(fn `UserConstructionScript`
  (`parent.UserConstructionScript`))