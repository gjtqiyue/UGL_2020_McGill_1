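; Player controller for a two-player networked game, handling lobby ready state, pausing and game over.
; Ready and pause requests run directly on authority or go through server events, updating the GameState ready count or toggling pause in the GameMode.
; Tick triggers game over when the locally controlled character and its partner are both down.
; Game over routes through server and multi events to load the GameOver level via GameInstance and reset both players.
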(event `self.ReceiveBeginPlay`
  (bind _asbp_game_state (cast `/Game/Blueprints/BP_GameState` (`GameplayStatics.GetGameState`)))
  (set `self.GameState` _asbp_game_state)
  (bind _asbp_game_mode (cast `/Game/Blueprints/BP_GameMode` (`GameplayStatics.GetGameMode`)))
  (set `self.GameMode` _asbp_game_mode))

(event `SetPlayerReady`
  ;[1 1 1] Lobby Ready State
  (if (`self.HasAuthority`)
    (`/Game/Blueprints/BP_GameState.SetNumReady` (`self.GameState`))
    (else
      (`self.SetPlayerReadyServer`))))

(event `SetPlayerReadyServer`
  ;[1 1 1] Lobby Ready State
  (`/Game/Blueprints/BP_GameState.SetNumReady` (`self.GameState`)))

(event `InputAction|Pause` :paused true
  (params (Key :type "Key Structure"))
  ;[1 1 1] Pausing game
  (:`Pressed`
    (`/Engine/EditorBlueprintResources/ActorMacros.Switch Has Authority`
      (:`Authority`
        (`/Game/Blueprints/BP_GameMode.TogglePause` (`self.GameMode`)))
      (:`Remote`
        (`self.PauseGameServer`)))))

(event `PauseGameServer`
  ;[1 1 1] Pausing game
  (`self.PauseGameMulti`))

(event `PauseGameMulti`
  ;[1 1 1] Pausing game
  (`/Engine/EditorBlueprintResources/ActorMacros.Switch Has Authority`
    (:`Authority`
      (`/Game/Blueprints/BP_GameMode.TogglePause` (`self.GameMode`)))))

(event `GameOverServer`
  ;[1 1 1] Game over
  (`self.GameOverMulti`))

(event `GameOver`
  ;[1 1 1] Game over
  (if (`KismetSystemLibrary.IsServer`)
    (`self.GameOverMulti`)
    (else
      (`self.GameOverServer`))))

(event `GameOverMulti`
  ;[1 1 1] Game over
  (`/Game/Blueprints/BP_GameInstance.LoadLevel` (cast `/Game/Blueprints/BP_GameInstance` (`GameplayStatics.GetGameInstance`) :!pure true) self "GameOver")
  (`KismetSystemLibrary.PrintString` "GAME OVER")
  (bind _asbp_character_base (cast `/Game/Blueprints/Characters/BP_CharacterBase` (`self.K2_GetPawn`)))
  (bind _otherplayer (`/Game/Blueprints/Characters/BP_CharacterBase.OtherPlayer` _asbp_character_base))
  (`/Engine/EditorBlueprintResources/StandardMacros.IsValid` _otherplayer
    (:`Is Valid`
      (`/Game/Blueprints/Characters/BP_CharacterBase.Reset Player` _asbp_character_base)
      (`/Game/Blueprints/Characters/BP_CharacterBase.Reset Player` _otherplayer))))

(event `self.ReceiveTick`
  (params (DeltaSeconds :type "Float (single-precision)"))
  ;[1 1 1] Game over
  (bind _asbp_character_base (cast `/Game/Blueprints/Characters/BP_CharacterBase` (`self.K2_GetPawn`)))
  (bind _otherplayer (`/Game/Blueprints/Characters/BP_CharacterBase.OtherPlayer` _asbp_character_base))
  (`/Engine/EditorBlueprintResources/StandardMacros.IsValid` _otherplayer
    (:`Is Valid`
      (if (and (`Pawn.IsLocallyControlled` _asbp_character_base) (and (`/Game/Blueprints/Characters/BP_CharacterBase.isDown` _asbp_character_base) (`/Game/Blueprints/Characters/BP_CharacterBase.isDown` _otherplayer)))
        (`self.GameOver`)))))

(fn `UserConstructionScript`)