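; Skill projectile actor that purifies and hits what it overlaps.
; On overlap it calls Purify on any BP_PurificationComponent of the other actor, then calls TakeDamage on BP_EnemyBase actors with zero damage, crediting the BP_Character_Girl found in the world.
; Despite its name, DamageDestroy never destroys the projectile; that happens when an overlap ends with an actor not tagged Player.
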(event `self.ReceiveActorBeginOverlap`
  (params (OtherActor :type "Actor Object Reference"))
  (`|ExecutionSequence`
    (:`then_0`
      (`self.PurifyCheck` OtherActor))
    (:`then_1`
      (`self.Damage Destroy` OtherActor))))

(event `self.ReceiveActorEndOverlap`
  (params (OtherActor :type "Actor Object Reference"))
  (if (not (`self.ActorHasTag` OtherActor "Player"))
    (`self.K2_DestroyActor`)))

(fn `Damage Destroy`
  (params (HitActor :type "Actor Object Reference"))
  (bind _asbp_enemy_base (cast `/Game/Blueprints/AI/BP_EnemyBase` HitActor))
  (if (`KismetSystemLibrary.IsValid` _asbp_enemy_base)
    (bind _returnvalue (`GameplayStatics.GetActorOfClass` "/Game/Blueprints/Characters/BP_Character_Girl.BP_Character_Girl_C"))
    (`/Game/Blueprints/AI/BP_EnemyBase.TakeDamage` _asbp_enemy_base 0.0 _returnvalue 0)
    (return)))

(fn `PurifyCheck`
  (params (HitActor :type "Actor Object Reference"))
  (bind _returnvalue (`self.GetComponentByClass` HitActor "/Game/Blueprints/Components/BP_PurificationComponent.BP_PurificationComponent_C"))
  (`/Engine/EditorBlueprintResources/StandardMacros.IsValid` _returnvalue
    (:`Is Valid`
      (`/Game/Blueprints/Components/BP_PurificationComponent.Purify` _returnvalue 1.0))))

(fn `UserConstructionScript`)