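; BP_Inter_Kidonly is an interactable object that only the girl character can bring into range.
; Its outer trigger's begin and end overlap events check for an exact BP_Character_Girl class match before calling OnPlayerInRange or OnPlayerLeaveRange.
; The Trigger event only prints a debug message, and the construction script defers to the parent.
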(event `self.OuterTrigger.OnComponentBeginOverlap`
  (params (OverlappedComponent :type "PrimitiveComponent Object Reference") (OtherActor :type "Actor Object Reference") (OtherComp :type "PrimitiveComponent Object Reference") (OtherBodyIndex :type Integer) (bFromSweep :type Boolean) (SweepResult :type "HitResult Structure (by ref)"))
  (if (== (`GameplayStatics.GetObjectClass` OtherActor) "/Game/Blueprints/Characters/BP_Character_Girl.BP_Character_Girl_C")
    (`self.OnPlayerInRange` null OtherActor)
    (`KismetSystemLibrary.PrintString` "Enter range")))

(event `self.OuterTrigger.OnComponentEndOverlap`
  (params (OverlappedComponent :type "PrimitiveComponent Object Reference") (OtherActor :type "Actor Object Reference") (OtherComp :type "PrimitiveComponent Object Reference") (OtherBodyIndex :type Integer))
  (if (== (`GameplayStatics.GetObjectClass` OtherActor) "/Game/Blueprints/Characters/BP_Character_Girl.BP_Character_Girl_C")
    (`self.OnPlayerLeaveRange` null OtherActor)))

(event `self.Trigger`
  (`KismetSystemLibrary.PrintString` "Trigger Kidonly object"))

(fn `UserConstructionScript`
  (`parent.UserConstructionScript`))