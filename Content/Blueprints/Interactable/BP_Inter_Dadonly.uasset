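; An interactable Blueprint, built on a parent class, that responds only to the Dad character.
; OuterTrigger overlaps filter on BP_Character_Dad, call the in-range and leave-range handlers, and toggle the UI through ShowUI and HideUI.
; ShowUI, HideUI and Trigger are empty here, and a debug string prints on entry.
; AddForce applies a large upward impulse to the mesh, but its call here is disconnected.
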(event `self.OuterTrigger.OnComponentBeginOverlap`
  (params (OverlappedComponent :type "PrimitiveComponent Object Reference") (OtherActor :type "Actor Object Reference") (OtherComp :type "PrimitiveComponent Object Reference") (OtherBodyIndex :type Integer) (bFromSweep :type Boolean) (SweepResult :type "HitResult Structure (by ref)"))
  (if (== (`GameplayStatics.GetObjectClass` OtherActor) "/Game/Blueprints/Characters/BP_Character_Dad.BP_Character_Dad_C")
    (`self.OnPlayerInRange` null OtherActor)
    (`KismetSystemLibrary.PrintString` "Enter range")
    (`self.ShowUI`)))

(event `self.OuterTrigger.OnComponentEndOverlap`
  (params (OverlappedComponent :type "PrimitiveComponent Object Reference") (OtherActor :type "Actor Object Reference") (OtherComp :type "PrimitiveComponent Object Reference") (OtherBodyIndex :type Integer))
  (if (== (`GameplayStatics.GetObjectClass` OtherActor) "/Game/Blueprints/Characters/BP_Character_Dad.BP_Character_Dad_C")
    (`self.OnPlayerLeaveRange` null OtherActor)
    (`self.HideUI`)))

(event `self.Trigger`)

(event `AddForce`
  (`PrimitiveComponent.AddImpulse` (`self.Mesh`) (0.0 0.0 7000000.0) "None" false))

(fn `HideUI`)

(fn `ShowUI`)

(fn `UserConstructionScript`
  (`parent.UserConstructionScript`))