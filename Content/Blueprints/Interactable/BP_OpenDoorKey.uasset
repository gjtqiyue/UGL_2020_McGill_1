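; Swinging door that opens when triggered while unlocked, or automatically as tracked enemies are destroyed.
; BeginPlay caches the mesh rotation and collects actors sharing the door's first tag into Enemy.
; Tick scans that list up to the first valid entry, opening for any invalid one regardless of Locked.
; OpenDoor switches on Opened to toggle collision and drive the DoorSwing timeline, which yaws the mesh from its initial rotation.
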(event `self.ReceiveBeginPlay`
  (set `self.InitialRotation` (`SceneComponent.RelativeRotation` (`self.Mesh`)))
  (bind _outactors (`GameplayStatics.GetAllActorsWithTag` (`|GetArrayItem` (`self.Tags`))))
  (for _array_element _outactors
    (`KismetArrayLibrary.Array_AddUnique` (`self.enemy`) _array_element)))

(event `self.Trigger`
  (if (`self.Locked`)
    (`KismetSystemLibrary.PrintString` "The door is locked")
    (elif (`self.IsOpen`)
      _
      (elif (not (`self.IsOpening`))
        (set `self.Opened` 1)
        (set `self.IsOpening` true)
        (`self.OpenDoor`)))))

(event `self.ReceiveTick`
  (params (DeltaSeconds :type "Float (single-precision)"))
  (set `self.killed` false)
  (for _array_element (`self.enemy`)
    (`/Engine/EditorBlueprintResources/StandardMacros.IsValid` _array_element :!label _label
      (:`Is Valid`
        (break))
      (:`Is Not Valid`
        (set `self.Opened` 1)
        (set `self.IsOpening` true)
        (`self.OpenDoor`))))
  (goto _label))

(event `OpenDoor`
  (switch `int` (`self.Opened`)
    (:`0`
      (`PrimitiveComponent.SetCollisionEnabled` (`self.Collider`) "QueryAndPhysics")
      (bind (_direction _openangle) (`Timeline|DoorSwing` :!via `Stop` :!label _label_2)
        (:`Update`
          (`SceneComponent.K2_SetRelativeRotation` (`self.Mesh`) (`KismetMathLibrary.ComposeRotators` (`KismetMathLibrary.MakeRotator` 0.0 0.0 _openangle) (`self.InitialRotation`)) false false))
        (:`Finished`
          (set `self.Opened` 0)
          (set `self.IsOpening` false)
          (bind _output_get (set `self.IsOpen` (not (`self.IsOpen`))))
          (if (not _output_get)
            (set `self.Opened` 0)
            (set `self.IsOpening` false)))))
    (:`1`
      (`PrimitiveComponent.SetCollisionEnabled` (`self.Collider`) "NoCollision")
      (goto _label_2))
    (:`2`
      (`PrimitiveComponent.SetCollisionEnabled` (`self.Collider`) "NoCollision")
      (goto _label_2 :!via `Reverse`))))

(fn `UserConstructionScript`
  (`parent.UserConstructionScript`))