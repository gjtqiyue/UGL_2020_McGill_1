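; A door that unlocks and opens once its linked purification targets are all purified.
; On BeginPlay it gathers the purification components of every actor sharing the door's first tag.
; Each Tick it polls those components, stopping at the first unpurified one, and sets the door opened and unlocked if all are purified and combat is not active.
; An empty component list never opens it.
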(event `self.ReceiveBeginPlay`
  (`parent.ReceiveBeginPlay`)
  (bind _outactors (`GameplayStatics.GetAllActorsWithTag` (`|GetArrayItem` (`self.Tags`))))
  (for _array_element _outactors
    (bind _returnvalue (`self.GetComponentByClass` _array_element "/Game/Blueprints/Components/BP_PurificationComponent.BP_PurificationComponent_C"))
    (`/Engine/EditorBlueprintResources/StandardMacros.IsValid` _returnvalue
      (:`Is Valid`
        (`KismetArrayLibrary.Array_AddUnique` (`self.PurificationComponents`) _returnvalue)))))

(event `self.ReceiveTick`
  (params (DeltaSeconds :type "Float (single-precision)"))
  (set `self.purified` false)
  (for _array_element (`self.PurificationComponents`)
    (bind _purified (`/Game/Blueprints/Components/BP_PurificationComponent.getPurified` _array_element))
    (bind _output_get (set `self.purified` _purified))
    (if (not _output_get)
      (break)))
  (if (and (`self.purified`) (not (`self.isInCombat`)))
    (set `self.Opened` 1)
    (set `self.Locked` false))
  (`parent.ReceiveTick` DeltaSeconds))

(fn `UserConstructionScript`
  (`parent.UserConstructionScript`))