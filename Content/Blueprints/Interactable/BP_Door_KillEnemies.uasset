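; A child door Blueprint that unlocks and opens once its linked enemies are gone.
; On BeginPlay it collects every BP_EnemyBase actor sharing the door's first tag into an Enemies list.
; Each tick it polls their validity, then unlocks and opens when none remain valid and combat is over.
; An empty list opens the door immediately, skipping the combat check.
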(event `self.ReceiveBeginPlay`
  (`parent.ReceiveBeginPlay`)
  (bind _outactors (`GameplayStatics.GetAllActorsWithTag` (`|GetArrayItem` (`self.Tags`))))
  (for _array_element _outactors
    (bind _asbp_enemy_base (cast `/Game/Blueprints/AI/BP_EnemyBase` _array_element))
    (`KismetArrayLibrary.Array_AddUnique` (`self.Enemies`) _asbp_enemy_base)))

(event `self.ReceiveTick`
  (params (DeltaSeconds :type "Float (single-precision)"))
  (set `self.purified` false)
  (if (!= (`KismetArrayLibrary.Array_Length` (`self.Enemies`)) 0)
    (for _array_element (`self.Enemies`)
      (`/Engine/EditorBlueprintResources/StandardMacros.IsValid` _array_element
        (:`Is Valid`
          (set `self.purified` false)
          (break))
        (:`Is Not Valid`
          (set `self.purified` true))))
    (if (and (`self.purified`) (not (`self.isInCombat`)))
      (set `self.Opened` 1 :!label _label)
      (set `self.Locked` false))
    (else
      (set `self.purified` true)
      (goto _label)))
  (`parent.ReceiveTick` DeltaSeconds))

(fn `UserConstructionScript`
  (`parent.UserConstructionScript`))