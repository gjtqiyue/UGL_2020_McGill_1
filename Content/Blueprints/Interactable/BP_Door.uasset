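; Interactable door that swings open when triggered unless locked, with optional auto-close after a short delay.
; Tick reads an Opened state to play, reverse or stop the DoorSwing timeline, which rotates the mesh from its initial rotation with collision off while moving.
; After a swing, it can bind to BP_Character_Dad's tutorial combat start event, which closes the door.
; ShowUI and HideUI pass the locked state to the BPW_Door feedback widget.
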(event `BindEvent`
  (bind _returnvalue (`GameplayStatics.GetActorOfClass` "/Game/Blueprints/Characters/BP_Character_Dad.BP_Character_Dad_C"))
  (`/Engine/EditorBlueprintResources/StandardMacros.IsValid` _returnvalue
    (:`Is Valid`
      (add `/Game/Blueprints/Characters/BP_CharacterBase.TutCombatStart` _returnvalue (delegate `CloseDoor`))
      (set `self.EventBind` true))))

(event `CloseDoor`
  (set `self.isInCombat` true)
  (set `self.Opened` 2))

(event `self.ReceiveBeginPlay`
  (set `self.InitialRotation` (`SceneComponent.RelativeRotation` (`self.Mesh`))))

(event `self.Trigger`
  (if (`self.Locked`)
    (`KismetSystemLibrary.PrintString` "The door is locked")
    (elif (`self.IsOpen`)
      _
      (elif (not (`self.IsOpening`))
        (set `self.Opened` 1)
        (set `self.IsOpening` true)))))

(event `self.ReceiveTick`
  (params (DeltaSeconds :type "Float (single-precision)"))
  (switch `int` (`self.Opened`)
    (:`0`
      (`PrimitiveComponent.SetCollisionEnabled` (`self.Collider`) "QueryAndPhysics")
      (bind (_direction _openangle) (`Timeline|DoorSwing` :!via `Stop` :!label _label)
        (:`Update`
          (`SceneComponent.K2_SetRelativeRotation` (`self.Mesh`) (`KismetMathLibrary.ComposeRotators` (`KismetMathLibrary.MakeRotator` 0.0 0.0 _openangle) (`self.InitialRotation`)) false false))
        (:`Finished`
          (set `self.Opened` 0)
          (set `self.IsOpening` false)
          (bind _output_get (set `self.IsOpen` (not (`self.IsOpen`))))
          (if _output_get
            (if (`self.AutomaticClose`)
              (`KismetSystemLibrary.Delay` 2.0)
              (set `self.Opened` 2)
              (set `self.IsOpening` true)
              (if (not (`self.EventBind`)) :!label _label_2
                (`self.BindEvent`)))
            (else
              (set `self.Opened` 0)
              (set `self.IsOpening` false)
              (goto _label_2))))))
    (:`1`
      (`PrimitiveComponent.SetCollisionEnabled` (`self.Collider`) "NoCollision")
      (goto _label))
    (:`2`
      (`PrimitiveComponent.SetCollisionEnabled` (`self.Collider`) "NoCollision")
      (goto _label :!via `Reverse`))))

(fn `HideUI`
  (`parent.HideUI`)
  (bind _asbpw_door (cast `/Game/Blueprints/Widgets/BPW_Door` (`WidgetComponent.GetUserWidgetObject` (`self.Feedback`))))
  (`/Game/Blueprints/Widgets/BPW_Door.HideLockUI` _asbpw_door (`self.Locked`)))

(fn `ShowUI`
  (`parent.ShowUI`)
  (bind _asbpw_door (cast `/Game/Blueprints/Widgets/BPW_Door` (`WidgetComponent.GetUserWidgetObject` (`self.Feedback`))))
  (`/Game/Blueprints/Widgets/BPW_Door.ShowLockUI` _asbpw_door (`self.Locked`)))

(fn `UserConstructionScript`
  (`parent.UserConstructionScript`))