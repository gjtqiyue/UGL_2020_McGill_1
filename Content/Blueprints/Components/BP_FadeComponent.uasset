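; Actor component that fades the owner's static mesh out and back in when its hidden state is toggled.
; Setup caches the mesh's first material and creates a dynamic instance of FadeMaterial, with Tick retrying while either is missing.
; Hiding swaps in the fade instance, Tick drives its Fade parameter through a curve at FadeRate, and the original material returns once fade-in completes.
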(event `self.ReceiveBeginPlay`
  (bind _returnvalue (`Actor.GetComponentByClass` (`self.GetOwner`) "/Script/Engine.StaticMeshComponent"))
  (bind _output (`|GetArrayItem` (`MeshComponent.GetMaterials` (`self.ParentMesh`))))
  ;[1 1 1] Set up parent and mesh
  (`/Engine/EditorBlueprintResources/StandardMacros.IsValid` _returnvalue :!label _label
    (:`Is Valid`
      (set `self.ParentMesh` _returnvalue)
      (bind _asmaterial (cast `Material` _output)
        (:`then`
          (set `self.BaseMaterial` _asmaterial))
        (:`CastFailed`
          (bind _asmaterial_instance (cast `MaterialInstance` _output))
          (set `self.BaseMaterialInstance` _asmaterial_instance)
          (set `self.isMaterialInstance` true)))
      (bind _returnvalue_2 (`KismetMaterialLibrary.CreateDynamicMaterialInstance` (`self.FadeMaterial`)))
      (set `self.FadeMaterialMID` _returnvalue_2))))

(event `SetParentMesh`
  ;[1 1 1] Set up parent and mesh
  (goto _label))

(event `self.ReceiveTick`
  (params (DeltaSeconds :type "Float (single-precision)"))
  (`/Engine/EditorBlueprintResources/StandardMacros.IsValid` (`self.FadeMaterialMID`)
    (:`Is Valid`
      ;[1 1 1] Nice fade in and out
      (`/Engine/EditorBlueprintResources/StandardMacros.IsValid` (`self.ParentMesh`)
        (:`Is Valid`
          (if (`self.Hidden`)
            (set `self.CurrentFadeTime` (`KismetMathLibrary.FClamp` (- (`self.CurrentFadeTime`) (* (`self.FadeRate`) DeltaSeconds))))
            (else
              (set `self.CurrentFadeTime` (`KismetMathLibrary.FClamp` (+ (* DeltaSeconds (`self.FadeRate`)) (`self.CurrentFadeTime`))))))
          (`MaterialInstanceDynamic.SetScalarParameterValue` (`self.FadeMaterialMID`) "Fade" (`CurveFloat.GetFloatValue` (`self.FadeCurve`) (`self.CurrentFadeTime`)))
          ;;[1 1 1] Bring back original material once fade done
          (if (and (not (`self.Hidden`)) (== (`self.CurrentFadeTime`) 1.0))
            (if (`self.isMaterialInstance`)
              (`PrimitiveComponent.SetMaterial` (`self.ParentMesh`) 0 (`self.BaseMaterialInstance`))
              (else
                (`PrimitiveComponent.SetMaterial` (`self.ParentMesh`) 0 (`self.BaseMaterial`))))))
        (:`Is Not Valid`
          (`self.SetParentMesh` :!label _label_2))))
    (:`Is Not Valid`
      (goto _label_2))))

(fn `Toggle hiden mesh`
  (params (hidden :type Boolean))
  (if (!= hidden (`self.Hidden`))
    (bind _output_get (set `self.Hidden` hidden))
    (if _output_get
      (`PrimitiveComponent.SetMaterial` (`self.ParentMesh`) 0 (`self.FadeMaterialMID`)))))