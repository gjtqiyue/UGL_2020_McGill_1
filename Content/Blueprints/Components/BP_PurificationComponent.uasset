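; Actor component that marks its owner with a ghost particle effect until it is purified.
; BeginPlay attaches the emitter to the owner's root; the authority hides its copy and initializes Health.
; Purify drains Health, and at zero DestroyParticle removes the effect and sets IsPurified, whose OnRep also destroys the particle.
; GetPurified exposes the state; logic to lower the spawn rate is unconnected.
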(event `self.ReceiveBeginPlay`
  (bind _returnvalue (`self.GetOwner`))
  (bind _returnvalue_2 (`GameplayStatics.SpawnEmitterAttached` "/Game/Assets/ParticleSystem/Ghost.Ghost" (`Actor.RootComponent` _returnvalue)))
  (bind _output_get (set `self.Particle` _returnvalue_2))
  (`FXSystemComponent.SetFloatParameter` _output_get "SpawnRate" (`self.SpawnRate`))
  (if (`Actor.HasAuthority` _returnvalue)
    (`SceneComponent.SetVisibility` (`self.Particle`) false false)
    (set `self.Health` (`self.MaxHealth`))))

(event `Purify`
  (params (Amount :type "Float (double-precision)"))
  (bind _output_get (set `self.Health` (`KismetMathLibrary.FClamp` (- (`self.Health`) Amount) 0.0 (`self.MaxHealth`))))
  (if (<= _output_get 0.0)
    (`self.DestroyParticle`)))

(event `DestroyParticle`
  (bind _particle (`self.Particle`))
  (if (`KismetSystemLibrary.IsValid` _particle)
    (`self.K2_DestroyComponent` _particle)
    (`KismetSystemLibrary.PrintString` "purified")
    (set `self.isPurified` true)))

(fn `getPurified`
  (returns (purified :type Boolean))
  (return (`self.isPurified`)))

(fn `OnRep_isPurified`
  (bind _particle (`self.Particle`))
  (`/Engine/EditorBlueprintResources/StandardMacros.IsValid` _particle
    (:`Is Valid`
      (`self.K2_DestroyComponent` _particle))))