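; DialogueTrigger is a one-shot trigger actor that starts dialogue once both the Father and Kid characters are inside its collision volume.
; Begin and end overlap events on the collision component read each BP_CharacterBase's role to set or clear a presence flag.
; Tick polls both flags, then calls TriggerDialogue on BP_GameInstance and destroys the actor.
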(event `self.ReceiveTick`
  (params (DeltaSeconds :type "Float (single-precision)"))
  (if (and (`self.IsDadIn`) (`self.IsKidIn`))
    (bind _asbp_game_instance (cast `/Game/Blueprints/BP_GameInstance` (`GameplayStatics.GetGameInstance`)))
    (`/Game/Blueprints/BP_GameInstance.TriggerDialogue` _asbp_game_instance)
    (`self.K2_DestroyActor`)))

(event `self.CollisionComponent.OnComponentBeginOverlap`
  (params (OverlappedComponent :type "PrimitiveComponent Object Reference") (OtherActor :type "Actor Object Reference") (OtherComp :type "PrimitiveComponent Object Reference") (OtherBodyIndex :type Integer) (bFromSweep :type Boolean) (SweepResult :type "HitResult Structure (by ref)"))
  (bind _asbp_character_base (cast `/Game/Blueprints/Characters/BP_CharacterBase` OtherActor))
  (switch `EPlayerRole` (`CharacterBase.CharacterRole` _asbp_character_base)
    (:`VE_Father`
      (set `self.IsDadIn` true))
    (:`VE_Girl`
      (set `self.IsKidIn` true))))

(event `self.CollisionComponent.OnComponentEndOverlap`
  (params (OverlappedComponent :type "PrimitiveComponent Object Reference") (OtherActor :type "Actor Object Reference") (OtherComp :type "PrimitiveComponent Object Reference") (OtherBodyIndex :type Integer))
  (bind _asbp_character_base (cast `/Game/Blueprints/Characters/BP_CharacterBase` OtherActor))
  (switch `EPlayerRole` (`CharacterBase.CharacterRole` _asbp_character_base)
    (:`VE_Father`
      (set `self.IsDadIn` false))
    (:`VE_Girl`
      (set `self.IsKidIn` false))))

(fn `UserConstructionScript`)