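; Tutorial trigger box that starts the first combat once both the Father and Kid characters have entered it.
; Overlaps set a flag per role; end-overlap only clears flags already false, so entries effectively latch.
; With both set, it calls TutCombatStart on every character, whose BeginPlay-bound handler sets StartFirstCombat in character state.
; The server then spawns the Tutorial enemy through BP_GameInstance and disables its trigger.
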(event `self.Box.OnComponentBeginOverlap`
  (params (OverlappedComponent :type "PrimitiveComponent Object Reference") (OtherActor :type "Actor Object Reference") (OtherComp :type "PrimitiveComponent Object Reference") (OtherBodyIndex :type Integer) (bFromSweep :type Boolean) (SweepResult :type "HitResult Structure (by ref)"))
  (if (`self.Enabled`)
    (bind _asbp_character_base (cast `/Game/Blueprints/Characters/BP_CharacterBase` OtherActor))
    (switch `EPlayerRole` (`CharacterBase.CharacterRole` _asbp_character_base)
      (:`VE_Father`
        (if (not (`self.IsDadIn`))
          (set `self.IsDadIn` true)
          (`self.TriggerEnterEvent` :!label _label)))
      (:`VE_Girl`
        (if (not (`self.IsGirlIn`))
          (set `self.IsGirlIn` true)
          (goto _label))))))

(event `TriggerEnterEvent`
  (if (and (`self.IsDadIn`) (`self.IsGirlIn`))
    (bind _outactors (`GameplayStatics.GetAllActorsOfClass` "/Game/Blueprints/Characters/BP_CharacterBase.BP_CharacterBase_C"))
    (for _array_element _outactors
      (`/Game/Blueprints/Characters/BP_CharacterBase.TutCombatStart` _array_element))
    (if (`KismetSystemLibrary.IsServer`)
      (bind _asbp_game_instance (cast `/Game/Blueprints/BP_GameInstance` (`GameplayStatics.GetGameInstance`)))
      (`/Game/Blueprints/BP_GameInstance.SpawnEnemy` _asbp_game_instance "Tutorial" (1700.0 0.0 0.0001) 0)
      (set `self.Enabled` false))))

(event `self.ReceiveBeginPlay`
  (bind _outactors (`GameplayStatics.GetAllActorsOfClass` "/Game/Blueprints/Characters/BP_CharacterBase.BP_CharacterBase_C"))
  (for _array_element _outactors
    (add `/Game/Blueprints/Characters/BP_CharacterBase.TutCombatStart` _array_element (delegate `SetCombatStart`))))

(event `self.Box.OnComponentEndOverlap`
  (params (OverlappedComponent :type "PrimitiveComponent Object Reference") (OtherActor :type "Actor Object Reference") (OtherComp :type "PrimitiveComponent Object Reference") (OtherBodyIndex :type Integer))
  (if (`self.Enabled`)
    (bind _asbp_character_base (cast `/Game/Blueprints/Characters/BP_CharacterBase` OtherActor))
    (switch `EPlayerRole` (`CharacterBase.CharacterRole` _asbp_character_base)
      (:`VE_Father`
        (if (not (`self.IsDadIn`))
          (set `self.IsDadIn` false)))
      (:`VE_Girl`
        (if (not (`self.IsGirlIn`))
          (set `self.IsGirlIn` false))))))

(event `SetCombatStart`
  (setmembers `/Game/Blueprints/Characters/State` :`StructRef` (`/Game/Blueprints/Characters/BP_CharacterBase.State` (stale `self.ReceiveBeginPlay` _array_element)) :`bStartFirstCombat` true))

(fn `UserConstructionScript`)