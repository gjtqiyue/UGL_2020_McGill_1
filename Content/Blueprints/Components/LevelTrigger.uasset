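; LevelTrigger is a level-transition volume that loads the next level once both the Father and Kid characters stand inside its box.
; Begin and end overlaps track each role's presence by casting to BP_CharacterBase, printing a waiting message on each entry.
; Each entry triggers a server-only check that calls LoadNextLevel on the cached BP_GameInstance and disables the trigger when both are present.
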(event `self.Box.OnComponentBeginOverlap`
  (params (OverlappedComponent :type "PrimitiveComponent Object Reference") (OtherActor :type "Actor Object Reference") (OtherComp :type "PrimitiveComponent Object Reference") (OtherBodyIndex :type Integer) (bFromSweep :type Boolean) (SweepResult :type "HitResult Structure (by ref)"))
  ;[1 1 1] Update player in or out boolean
  (if (`self.Enabled`)
    (bind _asbp_character_base (cast `/Game/Blueprints/Characters/BP_CharacterBase` OtherActor))
    (switch `EPlayerRole` (`CharacterBase.CharacterRole` _asbp_character_base)
      (:`VE_Father`
        (if (not (`self.IsDadIn`))
          (set `self.IsDadIn` true)
          (`KismetSystemLibrary.PrintString` "Waiting for the girl")
          (`self.TriggerEnterEvent` :!label _label)))
      (:`VE_Girl`
        (if (not (`self.IsGirlIn`))
          (set `self.IsGirlIn` true)
          (`KismetSystemLibrary.PrintString` "Waiting for the dad")
          (goto _label))))))

(event `TriggerEnterEvent`
  (if (`KismetSystemLibrary.IsServer`)
    (if (and (`self.IsDadIn`) (`self.IsGirlIn`))
      (`/Game/Blueprints/BP_GameInstance.LoadNextLevel` (`self.GameInstance`))
      (set `self.Enabled` false))))

(event `self.ReceiveBeginPlay`
  (bind _asbp_game_instance (cast `/Game/Blueprints/BP_GameInstance` (`GameplayStatics.GetGameInstance`)))
  (set `self.GameInstance` _asbp_game_instance))

(event `self.Box.OnComponentEndOverlap`
  (params (OverlappedComponent :type "PrimitiveComponent Object Reference") (OtherActor :type "Actor Object Reference") (OtherComp :type "PrimitiveComponent Object Reference") (OtherBodyIndex :type Integer))
  ;[1 1 1] Update player in or out boolean
  (if (`self.Enabled`)
    (bind _asbp_character_base (cast `/Game/Blueprints/Characters/BP_CharacterBase` OtherActor))
    (switch `EPlayerRole` (`CharacterBase.CharacterRole` _asbp_character_base)
      (:`VE_Father`
        (if (`self.IsDadIn`)
          (set `self.IsDadIn` false)))
      (:`VE_Girl`
        (if (`self.IsGirlIn`)
          (set `self.IsGirlIn` false))))))

(fn `UserConstructionScript`)