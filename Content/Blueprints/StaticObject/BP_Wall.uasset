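; BP_Wall is a wall actor that can spawn random furniture at its sides on BeginPlay when SpawnFurniture is set.
; SpawnRandomFurniture picks classes from FurnitureList and spawns at InnerSide, plus a separate pick at OuterSide unless OnlyInnerSide is set.
; Rotation follows each side's forward vector, additionally combined with InnerSide's world rotation in inner-only mode.
; The random index range includes the list length, so picks can fall out of bounds.
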(event `self.ReceiveBeginPlay`
  (if (`self.SpawnFurniture`)
    (`self.SpawnRandomFurniture`)))

(event `SpawnRandomFurniture`
  (bind _furniturelist (`self.FurnitureList`))
  (bind _furniturelist_2 (`self.FurnitureList`))
  (bind _innerside (`self.InnerSide`))
  (bind _furniturelist_3 (`self.FurnitureList`))
  (bind _innerside_2 (`self.InnerSide`))
  (bind _outerside (`self.OuterSide`))
  (bind (_returnvalue_location _returnvalue_rotation _returnvalue_scale) (`KismetMathLibrary.BreakTransform` (`SceneComponent.K2_GetComponentToWorld` _outerside)))
  (bind (_returnvalue_location_2 _returnvalue_rotation_2 _returnvalue_scale_2) (`KismetMathLibrary.BreakTransform` (`SceneComponent.K2_GetComponentToWorld` _innerside)))
  (bind (_returnvalue_location_3 _returnvalue_rotation_3 _returnvalue_scale_3) (`KismetMathLibrary.BreakTransform` (`SceneComponent.K2_GetComponentToWorld` _innerside_2)))
  (if (`self.OnlyInnerSide`)
    (`|SpawnActorFromClass` (`|GetArrayItem` _furniturelist_2 (`KismetMathLibrary.RandomIntegerInRange` 0 (`KismetArrayLibrary.Array_Length` _furniturelist_2))) (`KismetMathLibrary.MakeTransform` _returnvalue_location_2 (`KismetMathLibrary.ComposeRotators` (`KismetMathLibrary.Conv_VectorToRotator` (`SceneComponent.GetForwardVector` _innerside)) _returnvalue_rotation_2) _returnvalue_scale_2) "AdjustIfPossibleButAlwaysSpawn" "OverrideRootScale" null null)
    (else
      (`|SpawnActorFromClass` (`|GetArrayItem` _furniturelist_3 (`KismetMathLibrary.RandomIntegerInRange` 0 (`KismetArrayLibrary.Array_Length` _furniturelist_3))) (`KismetMathLibrary.MakeTransform` _returnvalue_location_3 (`KismetMathLibrary.Conv_VectorToRotator` (`SceneComponent.GetForwardVector` _innerside_2)) _returnvalue_scale_3) "AdjustIfPossibleButAlwaysSpawn" "OverrideRootScale" null null)
      (`|SpawnActorFromClass` (`|GetArrayItem` _furniturelist (`KismetMathLibrary.RandomIntegerInRange` 0 (`KismetArrayLibrary.Array_Length` _furniturelist))) (`KismetMathLibrary.MakeTransform` _returnvalue_location (`KismetMathLibrary.Conv_VectorToRotator` (`SceneComponent.GetForwardVector` _outerside)) _returnvalue_scale) "AdjustIfPossibleButAlwaysSpawn" "OverrideRootScale" null null))))

(fn `UserConstructionScript`)