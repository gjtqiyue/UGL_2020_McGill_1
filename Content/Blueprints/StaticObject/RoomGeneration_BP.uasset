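; RoomGeneration_BP is a static level actor that procedurally builds a room layout on the server at BeginPlay.
; It generates rooms from level corners and a room count, converts them to walls, and marks door walls.
; It spawns scaled door or plain wall actors relative to itself, skipping ignored positions.
; A test room decomposition prints debug counts, and the loop appending reserved rooms is disconnected.
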(event `self.ReceiveBeginPlay`
  (bind _testroom (`self.TestRoom`))
  (if (`KismetSystemLibrary.IsServer`)
    (bind _returnvalue (`self.GenerateRoomWalls` (`self.Level Corners`) (`self.numRooms`)))
    (`self.Create Walls` (`.rooms` (break `GeneratedLevel` _returnvalue)))
    (bind _returnvalue_2 (`LevelGenerationUsage.DecomposeRoom` _testroom))
    (`KismetSystemLibrary.PrintString` (`KismetStringLibrary.Conv_IntToString` (`KismetArrayLibrary.Array_Length` _returnvalue_2)))
    (`KismetSystemLibrary.PrintString` (`KismetStringLibrary.Conv_IntToString` (`KismetArrayLibrary.Array_Length` (`.corners` (break `Room` _testroom)))))))

(fn `Create Walls`
  (params (rooms :type "Array of Room Structure"))
  (locals (Walls :type "Array of Wall Structure") (ActorToSpawn :type "Actor Class Reference"))
  (bind _returnvalue (`LevelGenerationUsage.CreateLevelWallFromRooms` rooms))
  (bind _output_get (set `local.Walls` _returnvalue))
  (`LevelGenerationUsage.GenerateDoorWalls` _output_get)
  (for _array_element (`local.Walls`)
    (bind _returnvalue_2 (`LevelGenerationUsage.GetWallCreationTransforms` _array_element (`self.ScalingFactor`)))
    (bind _location (.location (`|GetArrayItem` _returnvalue_2)))
    (if (not (`KismetArrayLibrary.Array_Contains` (`self.WallsToIgnore`) (/ _location (`self.ScalingFactor`))))
      (if (`.hasDoor` (break `Wall` _array_element))
        (set `local.ActorToSpawn` (`self.DoorWallActor`))
        (else
          (set `local.ActorToSpawn` (`self.WallActor`))))
      (`|SpawnActorFromClass` (`local.ActorToSpawn`) (`KismetMathLibrary.MakeTransform` (+ _location (`self.K2_GetActorLocation`)) (.rotation (`|GetArrayItem` _returnvalue_2)) (.scale (`|GetArrayItem` _returnvalue_2))) "Undefined" "OverrideRootScale" null null))))

(fn `UserConstructionScript`)